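; BP_TimeManager is the city builder's economy tick, periodically updating the resource balances stored in GS_CityBuilderGameState.
; A self-rearming one-shot timer applies the population, research and production change values, clamped between zero and each maximum, then calls GameEndCheck.
; Each interval is recomputed from MaxTime and happiness, so higher happiness shortens the time between ticks.
; Disconnected happiness-indicator nodes remain unused.
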(event `self.ReceiveBeginPlay`
  (bind _currenttime (`self.CurrentTime`))
  (bind _asgs_city_builder_game_state (cast `/Game/CityBuilder/Core/Blueprints/GS_CityBuilderGameState` (`GameplayStatics.GetGameState`)))
  (set `self.GameState` _asgs_city_builder_game_state)
  (`KismetSystemLibrary.K2_SetTimerDelegate` (delegate `UpdateBalances`) _currenttime :!label _label)
  (`KismetSystemLibrary.PrintString` (`KismetStringLibrary.Conv_DoubleToString` _currenttime) true false (struct :`R` 0.23129 :`G` 1.0 :`A` 1.0)))

(event `UpdateBalances`
  (bind _gamestate (`self.GameState`))
  (bind _gamestate_2 (`self.GameState`))
  (bind _gamestate_3 (`self.GameState`))
  (bind _populationchange (`/Game/CityBuilder/Core/Blueprints/GS_CityBuilderGameState.PopulationChange` _gamestate))
  (bind _researchchange (`/Game/CityBuilder/Core/Blueprints/GS_CityBuilderGameState.ResearchChange` _gamestate_2))
  (bind _productionchange (`/Game/CityBuilder/Core/Blueprints/GS_CityBuilderGameState.ProductionChange` _gamestate_3))
  (set `self.CurrentTime` (- (- (`self.MaxTime`) 50.0) (`KismetMathLibrary.Conv_IntToDouble` (/ (`/Game/CityBuilder/Core/Blueprints/GS_CityBuilderGameState.HappinessPercent` (`self.GameState`)) 10))))
  (`|ExecutionSequence`
    (:`then_0`
      (if (not (== _populationchange 0))
        (set `/Game/CityBuilder/Core/Blueprints/GS_CityBuilderGameState.PopulationBalance` (`KismetMathLibrary.Clamp` (+ _populationchange (`/Game/CityBuilder/Core/Blueprints/GS_CityBuilderGameState.PopulationBalance` _gamestate)) 0 (`/Game/CityBuilder/Core/Blueprints/GS_CityBuilderGameState.PopulationMax` _gamestate)) _gamestate)))
    (:`then_1`
      (if (not (== _researchchange 0))
        (set `/Game/CityBuilder/Core/Blueprints/GS_CityBuilderGameState.ResearchBalance` (`KismetMathLibrary.Clamp` (+ _researchchange (`/Game/CityBuilder/Core/Blueprints/GS_CityBuilderGameState.ResearchBalance` _gamestate_2)) 0 (`/Game/CityBuilder/Core/Blueprints/GS_CityBuilderGameState.ResearchMax` _gamestate_2)) _gamestate_2)))
    (:`then_2`
      (if (not (== _productionchange 0))
        (set `/Game/CityBuilder/Core/Blueprints/GS_CityBuilderGameState.ProductionBalance` (`KismetMathLibrary.Clamp` (+ _productionchange (`/Game/CityBuilder/Core/Blueprints/GS_CityBuilderGameState.ProductionBalance` _gamestate_3)) 0 (`/Game/CityBuilder/Core/Blueprints/GS_CityBuilderGameState.ProductionMax` _gamestate_3)) _gamestate_3)))
    (:`then_3`
      (`/Game/CityBuilder/Core/Blueprints/Libraries/BFL_GlobalFunctionLibrary.GameEndCheck`))
    (:`then_4`
      (goto _label))))

(fn `UserConstructionScript`)