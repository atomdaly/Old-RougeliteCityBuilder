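; City builder spawner actor that scatters random resource actors across the map shortly after BeginPlay.
; SpawnResources repeatedly picks random XY points snapped to a grid and line-traces down from above to find a surface.
; SpawnCheckTraces validates each hit with four short downward corner traces, all needing a blocking hit beyond a minimum distance.
; Valid points spawn a random class from the Resources array; both trace stages draw debug lines.
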(event `self.ReceiveBeginPlay`
  (`KismetSystemLibrary.Delay` 0.1)
  (`self.SpawnResources`))

(fn `SpawnCheckTraces`
  (params (MainHitLocation :type "Vector Structure"))
  (returns (`bValidLocation?` :type Boolean))
  (bind _tracelocation (`self.TraceLocation`))
  (bind _returnvalue (* _tracelocation -1.0))
  (for _index (range 4)
    (bind _returnvalue_2 (+ MainHitLocation (`KismetMathLibrary.MakeVector` (select `int` _index :`0` _returnvalue :`1` _tracelocation :`2` _tracelocation :`3` _returnvalue) (select `int` _index :`0` _tracelocation :`1` _tracelocation :`2` _returnvalue :`3` _returnvalue) 25.0)))
    (bind _outhit (`KismetSystemLibrary.LineTraceSingle` :`Start` _returnvalue_2 :`End` (- _returnvalue_2 (0.0 0.0 35.0)) :`TraceChannel` "TraceTypeQuery1" :`DrawDebugType` "ForDuration" :`TraceColor` (struct :`R` 0.848742 :`B` 1.0 :`A` 1.0) :`TraceHitColor` (struct :`R` 1.0 :`G` 0.861242 :`A` 1.0) :`DrawTime` 10.0))
    (bind (_bblockinghit _binitialoverlap _time _distance) (`GameplayStatics.BreakHitResult` _outhit))
    (if (and _bblockinghit (> _distance 10.0))
      (bind _returnvalue_3 (== _index 3))
      (if _returnvalue_3
        (return _returnvalue_3))
      (else
        (return false)))))

(fn `SpawnResources`
  (bind _returnvalue (`KismetMathLibrary.RandomFloatInRange` -6000.0 6000.0))
  (bind _returnvalue_2 (`KismetMathLibrary.RandomFloatInRange` -6000.0 6000.0))
  (bind _returnvalue_3 (mod _returnvalue 250.0))
  (bind _returnvalue_4 (mod _returnvalue_2 250.0))
  (bind _returnvalue_5 (- _returnvalue _returnvalue_3))
  (bind _returnvalue_6 (- _returnvalue_2 _returnvalue_4))
  (bind _returnvalue_7 (select `bool` (< _returnvalue_3 125.0) :`false` _returnvalue_5 :`true` (+ _returnvalue_5 250.0)))
  (bind _returnvalue_8 (select `bool` (< _returnvalue_4 125.0) :`false` _returnvalue_6 :`true` (+ _returnvalue_6 250.0)))
  (for _ (range 26)
    (bind _outhit (`KismetSystemLibrary.LineTraceSingle` :`Start` (`KismetMathLibrary.MakeVector` _returnvalue_8 _returnvalue_7 5000.0) :`End` (`KismetMathLibrary.MakeVector` _returnvalue_8 _returnvalue_7 250.0) :`TraceChannel` "TraceTypeQuery3" :`DrawDebugType` "ForDuration" :`TraceColor` (struct :`R` 0.733938 :`G` 1.0 :`A` 1.0) :`TraceHitColor` (struct :`R` 1.0 :`G` 0.308904 :`A` 1.0)))
    (bind (_bblockinghit _binitialoverlap _time _distance _location) (`GameplayStatics.BreakHitResult` _outhit))
    (if _bblockinghit
      (bind _bvalidlocation_ (`self.SpawnCheckTraces` _location))
      (if _bvalidlocation_
        (`|SpawnActorFromClass` (`KismetArrayLibrary.Array_Random` (`self.Resources`)) (`KismetMathLibrary.MakeTransform` _location (`KismetMathLibrary.MakeRotator` 0.0)) "Undefined" "OverrideRootScale" null null)))))

(fn `UserConstructionScript`)