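; Player controller for the city builder that owns the HUD, pause, build and research menus, and mouse-driven building placement.
; Placement mode moves a dummy building with a per-type placeable component along a cursor trace.
; Clicking checks cost and validity, spawns BP_PlacedBuilding, then applies data table costs and bonuses to the GameState.
; It also randomizes terrain colors through a parameter collection and has debug keys; random town-center spawning is disconnected.
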(event `self.ReceiveBeginPlay`
  (bind _returnvalue (`|CreateWidget` "/Game/CityBuilder/UI/Blueprints/HUD/WBP_HUD.WBP_HUD_C"))
  (bind _output_get (set `self.HUD` _returnvalue))
  (`UserWidget.AddToViewport` _output_get 0)
  (`self.RandomizeTerrainColors`)
  (bind _asgs_city_builder_game_state (cast `/Game/CityBuilder/Core/Blueprints/GS_CityBuilderGameState` (`GameplayStatics.GetGameState`)))
  (set `self.GameState` _asgs_city_builder_game_state))

(event `self.ReceiveTick`
  (params (DeltaSeconds :type "Float (single-precision)"))
  (if (`self.bPlacementModeEnabled?`)
    (`self.UpdatePlacement`)))

(event `OpenPauseMenu`
  (bind _returnvalue (`GameplayStatics.GetPlayerController` 0))
  (bind _foundwidgets (`WidgetBlueprintLibrary.GetAllWidgetsOfClass` "/Script/UMG.UserWidget"))
  (for _array_element _foundwidgets
    (`/Engine/EditorBlueprintResources/StandardMacros.IsValid` _array_element
      (:`Is Valid`
        (`Widget.SetVisibility` _array_element "Hidden"))))
  (`GameplayStatics.SetGamePaused` true)
  (bind _returnvalue_2 (`|CreateWidget` "/Game/CityBuilder/UI/Blueprints/PauseMenu/WBP_PauseMenu.WBP_PauseMenu_C"))
  (bind _output_get (set `self.PauseMenuRef` _returnvalue_2))
  (`UserWidget.AddToViewport` _output_get 0)
  (set `self.bPauseMenuOpen?` true)
  (`self.DisableInput` (`GameplayStatics.GetPlayerPawn` 0) _returnvalue)
  (set `PlayerController.bShowMouseCursor` (not (`self.bGamepadKey?`)) _returnvalue))

(event `ClosePauseMenu`
  (bind _foundwidgets (`WidgetBlueprintLibrary.GetAllWidgetsOfClass` "/Game/AutoSettings/SettingsUI.SettingsUI_C"))
  (bind _output (`|GetArrayItem` _foundwidgets))
  (`/Engine/EditorBlueprintResources/StandardMacros.IsValid` _output
    (:`Is Valid`
      (`Widget.RemoveFromParent` _output)
      (`self.OpenPauseMenu`))
    (:`Is Not Valid`
      (`Widget.RemoveFromParent` (`self.PauseMenuRef`))
      (`GameplayStatics.SetGamePaused` false)
      (set `self.bPauseMenuOpen?` false)
      (set `PlayerController.bShowMouseCursor` (not (`self.bGamepadKey?`)) (`GameplayStatics.GetPlayerController` 0))
      (`self.EnableInput` (`GameplayStatics.GetPlayerPawn` 0) (`GameplayStatics.GetPlayerController` 0))
      (bind _foundwidgets_2 (`WidgetBlueprintLibrary.GetAllWidgetsOfClass` "/Script/UMG.UserWidget"))
      (for _array_element _foundwidgets_2
        (`/Engine/EditorBlueprintResources/StandardMacros.IsValid` _array_element
          (:`Is Valid`
            (`Widget.SetVisibility` _array_element "SelfHitTestInvisible")))))))

(event `InputAction|Back/Pause` :paused true
  (params (Key :type "Key Structure"))
  (bind _hud (`self.HUD`))
  (bind _selectedactor (`/Game/CityBuilder/UI/Blueprints/HUD/WBP_HUD.SelectedActor` _hud))
  (:`Pressed`
    (set `self.bGamepadKey?` (`KismetInputLibrary.Key_IsGamepadKey` Key))
    (bind _foundwidgets (`WidgetBlueprintLibrary.GetAllWidgetsOfClass` "/Game/CityBuilder/UI/Blueprints/HUD/WBP_ModalPopUp.WBP_ModalPopUp_C" false))
    (bind _output (`|GetArrayItem` _foundwidgets))
    (`/Engine/EditorBlueprintResources/StandardMacros.IsValid` _output
      (:`Is Valid`
        (`Widget.RemoveFromParent` _output))
      (:`Is Not Valid`
        (if (`self.bBuildMenuOpen?`)
          (`/Game/CityBuilder/UI/Blueprints/HUD/WBP_BuildMenu.DisableAll` (`/Game/CityBuilder/UI/Blueprints/HUD/WBP_HUD.WBP_BuildMenu` _hud))
          (else
            (switch `int` (`/Game/CityBuilder/UI/Blueprints/HUD/WBP_HUD.OpenMenuIndex` _hud)
              (:`Default`
                (if (`self.bPauseMenuOpen?`) :!label _label
                  (`self.ClosePauseMenu`)
                  (else
                    (`self.OpenPauseMenu`)
                    (`self.SetPlacementModeEnabled` false))))
              (:`0`
                (goto _label))
              (:`1`
                (`/Engine/EditorBlueprintResources/StandardMacros.IsValid` _selectedactor
                  (:`Is Valid`
                    (`/Game/CityBuilder/Core/Blueprints/Components/BPC_SelectableComp.Deselected` (`self.GetComponentByClass` _selectedactor "/Game/CityBuilder/Core/Blueprints/Components/BPC_SelectableComp.BPC_SelectableComp_C")))))
              (:`2`
                (`/Game/CityBuilder/UI/Blueprints/HUD/WBP_HUD.ToggleResearchMenu` _hud)))))))))

(event `ToggleBuildMenu`
  ;[1 1 1] Menus
  (if (`self.bBuildMenuOpen?`)
    (set `self.bBuildMenuOpen?` false)
    (`self.SetPlacementModeEnabled` false)
    (else
      (if (`self.bResearchMenuOpen?`)
        (`/Game/CityBuilder/UI/Blueprints/HUD/WBP_HUD.CloseResearchMenu` (`self.HUD`))
        (set `self.bResearchMenuOpen?` false)
        (`self.EnableInput` (`GameplayStatics.GetPlayerPawn` 0) (`GameplayStatics.GetPlayerController` 0)))
      (set `self.bBuildMenuOpen?` true))))

(event `InputAction|OpenBuildMenu`
  (params (Key :type "Key Structure")))

(event `ToggleResearchMenu`
  (bind _returnvalue (`GameplayStatics.GetPlayerPawn` 0))
  (bind _returnvalue_2 (`GameplayStatics.GetPlayerController` 0))
  (bind _hud (`self.HUD`))
  ;[1 1 1] Menus
  (if (`self.bResearchMenuOpen?`)
    (`/Game/CityBuilder/UI/Blueprints/HUD/WBP_HUD.ToggleResearchMenu` _hud)
    (set `self.bResearchMenuOpen?` false)
    (`self.EnableInput` _returnvalue _returnvalue_2)
    (else
      (if (`self.bBuildMenuOpen?`)
        (set `self.bBuildMenuOpen?` false)
        (`self.SetPlacementModeEnabled` false))
      (`/Game/CityBuilder/UI/Blueprints/HUD/WBP_HUD.ToggleResearchMenu` _hud)
      (set `self.bResearchMenuOpen?` true)
      (`self.DisableInput` _returnvalue _returnvalue_2))))

(event `InputAction|OpenResearchMenu`
  (params (Key :type "Key Structure"))
  ;[1 1 1] Menus
  (:`Pressed`
    (`self.ToggleResearchMenu`)))

(event `InputAction|FocusOnObject`
  (params (Key :type "Key Structure"))
  (bind _selectedactor (`/Game/CityBuilder/UI/Blueprints/HUD/WBP_HUD.SelectedActor` (`self.HUD`)))
  (:`Pressed`
    (`/Engine/EditorBlueprintResources/StandardMacros.IsValid` _selectedactor
      (:`Is Valid`
        (`self.K2_SetActorLocation` (`GameplayStatics.GetPlayerPawn` 0) (`self.K2_GetActorLocation` _selectedactor) false false)))))

(event `InputAxis|RotateBuilding`
  (params (AxisValue :type "Float (single-precision)"))
  (bind _placeableactor (`self.PlaceableActor`))
  (`/Engine/EditorBlueprintResources/StandardMacros.IsValid` _placeableactor
    (:`Is Valid`
      (`self.K2_SetActorRotation` _placeableactor (`KismetMathLibrary.MakeRotator` (.roll (`self.K2_GetActorRotation` _placeableactor)) (.pitch (`self.K2_GetActorRotation` _placeableactor)) (+ (* AxisValue (`self.BuildingRotationSpeed`)) (.yaw (`self.K2_GetActorRotation` _placeableactor)))) false))))

(event `InputAction|MouseLeftClick`
  (params (Key :type "Key Structure"))
  (:`Pressed`
    (if (`self.bPlacementModeEnabled?`)
      (`self.SpawnBuilding`)
      (else
        (`self.DisableWidgetsOnClickOff`)))))

(event `InputAction|SlowBuildingRotation`
  (params (Key :type "Key Structure"))
  (:`Pressed`
    (set `self.BuildingRotationSpeed` 0.5))
  (:`Released`
    (set `self.BuildingRotationSpeed` 2.0)))

(event `Key|AnyKey` :consume false
  (params (Key :type "Key Structure"))
  ;[1 1 1] Update player's Key Group when input is pressedi.e. When you press a button on the gamepad, all the prompts update to reflect the gamepad mappings instead of the keyboard mappings
  (:`Pressed`
    (`InputMappingManager.SetPlayerKeyGroupStatic` self (`AutoSettingsInputProjectConfig.GetKeyGroupStatic` Key))))

(event `Key|Zero`
  (params (Key :type "Key Structure"))
  (:`Pressed`
    (`self.RandomizeTerrainColors`)))

(event `Key|One`
  (params (Key :type "Key Structure"))
  (bind _gamestate (`self.GameState`))
  (:`Pressed`
    (set `/Game/CityBuilder/Core/Blueprints/GS_CityBuilderGameState.PopulationBalance` 1000 _gamestate)
    (set `/Game/CityBuilder/Core/Blueprints/GS_CityBuilderGameState.ResearchBalance` 1000 _gamestate)
    (set `/Game/CityBuilder/Core/Blueprints/GS_CityBuilderGameState.ProductionBalance` 1000 _gamestate)))

(event `Key|Two`
  (params (Key :type "Key Structure"))
  (:`Pressed`
    (`GameplayStatics.SetGamePaused` true)
    (bind _returnvalue (`|CreateWidget` "/Game/CityBuilder/UI/Blueprints/HUD/WBP_GameOverScreen.WBP_GameOverScreen_C"))
    (`UserWidget.AddToViewport` _returnvalue 0)))

(event `Key|Nine`
  (params (Key :type "Key Structure"))
  (:`Pressed`
    (bind _returnvalue (`GameplayStatics.GetCurrentLevelName` true))
    (`GameplayStatics.OpenLevel` (`KismetStringLibrary.Conv_StringToName` _returnvalue))))

(fn `DisableWidgetsOnClickOff`
  (bind (_worldlocation _worlddirection) (`self.DeprojectMousePositionToWorld`))
  (bind _hud (`self.HUD`))
  (bind _selectedactor (`/Game/CityBuilder/UI/Blueprints/HUD/WBP_SelectedBuildingMenu.SelectedActor` (`/Game/CityBuilder/UI/Blueprints/HUD/WBP_HUD.WBP_SelectedBuildingMenu` _hud)))
  (bind _selectedactor_2 (`/Game/CityBuilder/UI/Blueprints/HUD/WBP_SelectedResourceMenu.SelectedActor` (`/Game/CityBuilder/UI/Blueprints/HUD/WBP_HUD.WBP_SelectedResourceMenu` _hud)))
  (bind _outhit (`KismetSystemLibrary.LineTraceSingle` _worldlocation (+ _worldlocation (* _worlddirection 25000.0)) "TraceTypeQuery1"))
  (bind (_bblockinghit _binitialoverlap _time _distance _location _impactpoint _normal _impactnormal _physmat _hitactor) (`GameplayStatics.BreakHitResult` _outhit))
  (if _bblockinghit
    (if (not (`self.ActorHasTag` _hitactor "Selectable"))
      (set `self.bResearchMenuOpen?` true)
      (`/Engine/EditorBlueprintResources/StandardMacros.IsValid` _selectedactor
        (:`Is Valid`
          (`/Game/CityBuilder/Core/Blueprints/Components/BPC_SelectableComp.Deselected` (`self.GetComponentByClass` _selectedactor "/Game/CityBuilder/Core/Blueprints/Components/BPC_SelectableComp.BPC_SelectableComp_C")))
        (:`Is Not Valid`
          (`/Engine/EditorBlueprintResources/StandardMacros.IsValid` _selectedactor_2
            (:`Is Valid`
              (`/Game/CityBuilder/Core/Blueprints/Components/BPC_SelectableComp.Deselected` (`self.GetComponentByClass` _selectedactor_2 "/Game/CityBuilder/Core/Blueprints/Components/BPC_SelectableComp.BPC_SelectableComp_C")))
            (:`Is Not Valid`
              _))))
      (`/Game/CityBuilder/UI/Blueprints/HUD/WBP_BuildMenu.DisableAll` (`/Game/CityBuilder/UI/Blueprints/HUD/WBP_HUD.WBP_BuildMenu` (`self.HUD`))))))

(fn `GetBuildingMesh`
  (returns (Mesh :type "StaticMesh Object Reference"))
  (return (select `/Game/CityBuilder/Core/Data/Enums/E_BuildingTypes` (`self.PlaceableBuildingType`) :`NewEnumerator0` (select `int` (`KismetMathLibrary.RandomIntegerInRange` 0 2) :`0` "/Game/CityBuilder/Art/3D/Environment/Buildings/SM_House_01.SM_House_01" :`1` "/Game/CityBuilder/Art/3D/Environment/Buildings/SM_House_02.SM_House_02" :`2` "/Game/CityBuilder/Art/3D/Environment/Buildings/SM_House_03.SM_House_03" :!type "StaticMesh Object Reference") :`NewEnumerator1` "/Game/CityBuilder/Art/3D/Environment/Buildings/SM_Mine_01.SM_Mine_01" :`NewEnumerator2` "/Game/CityBuilder/Art/3D/Environment/Buildings/SM_Farm_01.SM_Farm_01" :`NewEnumerator3` "/Game/CityBuilder/Art/3D/Environment/Buildings/SM_Dock_01.SM_Dock_01" :`NewEnumerator4` "/Game/CityBuilder/Art/3D/Environment/Buildings/SM_Lumbermill_01.SM_Lumbermill_01" :`NewEnumerator5` "/Game/CityBuilder/Art/3D/Blockout/SM_Cube.SM_Cube" :`NewEnumerator6` "/Game/CityBuilder/Art/3D/Environment/Buildings/SM_Market_01.SM_Market_01" :`NewEnumerator7` "/Game/CityBuilder/Art/3D/Environment/Buildings/SM_Blacksmith_01.SM_Blacksmith_01" :`NewEnumerator8` "/Game/CityBuilder/Art/3D/Environment/Buildings/SM_Tailor_01.SM_Tailor_01" :`NewEnumerator9` "/Game/CityBuilder/Art/3D/Environment/Buildings/SM_Tavern_01.SM_Tavern_01" :`NewEnumerator10` "/Game/CityBuilder/Art/3D/Blockout/SM_Cube.SM_Cube" :`NewEnumerator11` "/Game/CityBuilder/Art/3D/Blockout/SM_Cube.SM_Cube" :`NewEnumerator12` "/Game/CityBuilder/Art/3D/Blockout/SM_Cube.SM_Cube" :`NewEnumerator13` "/Game/CityBuilder/Art/3D/Blockout/SM_Cube.SM_Cube" :`NewEnumerator14` "/Game/CityBuilder/Art/3D/Blockout/SM_Cube.SM_Cube" :`NewEnumerator15` "/Game/CityBuilder/Art/3D/Blockout/SM_Cube.SM_Cube" :`NewEnumerator16` "/Game/CityBuilder/Art/3D/Blockout/SM_Cube.SM_Cube" :`NewEnumerator17` "/Game/CityBuilder/Art/3D/Blockout/SM_Cube.SM_Cube" :`NewEnumerator18` "/Game/CityBuilder/Art/3D/Environment/Buildings/SM_TradingPost_01.SM_TradingPost_01" :`NewEnumerator19` "/Game/CityBuilder/Art/3D/Blockout/SM_Cube.SM_Cube")))

(fn `RandomizeTerrainColors`
  (bind _terraincolorindex (`self.TerrainColorIndex`))
  (set `self.TerrainColorIndex` (`KismetMathLibrary.RandomIntegerInRange` 0 4))
  (`KismetMaterialLibrary.SetVectorParameterValue` "/Game/StylizedPaintedNature/Data/MPC_PN_GlobalSettings.MPC_PN_GlobalSettings" "GrassColour" (select `int` _terraincolorindex :`0` (struct :`R` 0.339727 :`G` 0.527115 :`B` 0.079067 :`A` 1.0) :`1` (struct :`R` 0.102475 :`G` 0.527115 :`B` 0.079067 :`A` 1.0) :`2` (struct :`R` 0.496933 :`G` 0.168269 :`B` 0.068478 :`A` 1.0) :`3` (struct :`R` 0.55834 :`G` 0.346704 :`B` 0.0865 :`A` 1.0) :`4` (struct :`R` 0.177888 :`G` 0.386429 :`B` 0.015996 :`A` 1.0) :!type "LinearColor Structure"))
  (`KismetMaterialLibrary.SetVectorParameterValue` "/Game/StylizedPaintedNature/Data/MPC_PN_GlobalSettings.MPC_PN_GlobalSettings" "CliffColor" (select `int` _terraincolorindex :`0` (struct :`R` 0.160963 :`G` 0.20949 :`B` 0.265625 :`A` 1.0) :`1` (struct :`R` 0.04653 :`G` 0.066931 :`B` 0.093059 :`A` 1.0) :`2` (struct :`R` 0.093059 :`G` 0.071966 :`B` 0.055835 :`A` 1.0) :`3` (struct :`R` 0.467784 :`G` 0.212231 :`B` 0.107023 :`A` 1.0) :`4` (struct :`R` 0.723055 :`G` 0.412543 :`B` 0.23074 :`A` 1.0) :!type "LinearColor Structure")))

(fn `SetPlacementModeEnabled`
  (params (`bIsEnabled?` :type Boolean))
  (bind _placeableactor (`self.PlaceableActor`))
  (if (== `bIsEnabled?` (`self.bPlacementModeEnabled?`))
    (return)
    (else
      (bind _output_get (set `self.bPlacementModeEnabled?` `bIsEnabled?`))
      (if _output_get
        (bind _returnvalue (`|SpawnActorFromClass` (`self.PlaceableActorClass`) (`KismetMathLibrary.MakeTransform` (0.0 0.0 -10000.0)) "AlwaysSpawn" "OverrideRootScale" null null))
        (bind _output_get_2 (set `self.PlaceableActor` _returnvalue))
        (bind _asbp_dummy_building (cast `/Game/CityBuilder/Core/Blueprints/Actors/Buidings/BP_DummyBuilding` _output_get_2))
        (bind _output_get_3 (set `self.BuildingMesh` (`self.GetBuildingMesh`)))
        (`StaticMeshComponent.SetStaticMesh` (`/Game/CityBuilder/Core/Blueprints/Actors/Buidings/BP_DummyBuilding.BuidingMesh` _asbp_dummy_building) _output_get_3)
        (`|AddComponentByClass` _output_get_2 (select `/Game/CityBuilder/Core/Data/Enums/E_BuildingTypes` (`self.PlaceableBuildingType`) :`NewEnumerator0` "/Game/CityBuilder/Core/Blueprints/Components/PlaceableComps/BPC_Placeable_House.BPC_Placeable_House_C" :`NewEnumerator1` "/Game/CityBuilder/Core/Blueprints/Components/PlaceableComps/BPC_Placeable_Mine.BPC_Placeable_Mine_C" :`NewEnumerator2` "/Game/CityBuilder/Core/Blueprints/Components/PlaceableComps/BPC_Placeable_Farm.BPC_Placeable_Farm_C" :`NewEnumerator3` "/Game/CityBuilder/Core/Blueprints/Components/PlaceableComps/BPC_Placeable_Dock.BPC_Placeable_Dock_C" :`NewEnumerator4` "/Game/CityBuilder/Core/Blueprints/Components/PlaceableComps/BPC_Placeable_LumberMill.BPC_Placeable_LumberMill_C" :`NewEnumerator5` "/Game/CityBuilder/Core/Blueprints/Components/BPC_PlaceableComp.BPC_PlaceableComp_C" :`NewEnumerator6` "/Game/CityBuilder/Core/Blueprints/Components/PlaceableComps/BPC_Placeable_Farm.BPC_Placeable_Farm_C" :`NewEnumerator7` "/Game/CityBuilder/Core/Blueprints/Components/BPC_PlaceableComp.BPC_PlaceableComp_C" :`NewEnumerator8` "/Game/CityBuilder/Core/Blueprints/Components/BPC_PlaceableComp.BPC_PlaceableComp_C" :`NewEnumerator9` "/Game/CityBuilder/Core/Blueprints/Components/BPC_PlaceableComp.BPC_PlaceableComp_C" :`NewEnumerator10` "/Game/CityBuilder/Core/Blueprints/Components/BPC_PlaceableComp.BPC_PlaceableComp_C" :`NewEnumerator11` "/Game/CityBuilder/Core/Blueprints/Components/BPC_PlaceableComp.BPC_PlaceableComp_C" :`NewEnumerator12` "/Game/CityBuilder/Core/Blueprints/Components/BPC_PlaceableComp.BPC_PlaceableComp_C" :`NewEnumerator13` "/Game/CityBuilder/Core/Blueprints/Components/BPC_PlaceableComp.BPC_PlaceableComp_C" :`NewEnumerator14` "/Game/CityBuilder/Core/Blueprints/Components/BPC_PlaceableComp.BPC_PlaceableComp_C" :`NewEnumerator15` "/Game/CityBuilder/Core/Blueprints/Components/BPC_PlaceableComp.BPC_PlaceableComp_C" :`NewEnumerator16` "/Game/CityBuilder/Core/Blueprints/Components/BPC_PlaceableComp.BPC_PlaceableComp_C" :`NewEnumerator17` "/Game/CityBuilder/Core/Blueprints/Components/BPC_PlaceableComp.BPC_PlaceableComp_C" :`NewEnumerator18` "/Game/CityBuilder/Core/Blueprints/Components/BPC_PlaceableComp.BPC_PlaceableComp_C" :`NewEnumerator19` "/Game/CityBuilder/Core/Blueprints/Components/BPC_PlaceableComp.BPC_PlaceableComp_C" :!type "ActorComponent Class Reference"))
        (return)
        (else
          (`/Engine/EditorBlueprintResources/StandardMacros.IsValid` _placeableactor
            (:`Is Valid`
              (`self.K2_DestroyActor` _placeableactor))))))))

(fn `SpawnBuilding`
  (bind _gamestate (`self.GameState`))
  (bind _gamestate_2 (`self.GameState`))
  (bind _returnvalue (`self.GetComponentByClass` (`self.PlaceableActor`) "/Game/CityBuilder/Core/Blueprints/Components/BPC_PlaceableComp.BPC_PlaceableComp_C"))
  (`/Engine/EditorBlueprintResources/StandardMacros.IsValid` _returnvalue
    (:`Is Valid`
      (bind _output (`self.CanAfford?`)
        (:`true`
          (if _output
            (if (`/Game/CityBuilder/Core/Blueprints/Components/BPC_PlaceableComp.bIsPlacementValid?` _returnvalue)
              (bind _returnvalue_2 (`|SpawnActorFromClass` "/Game/CityBuilder/Core/Blueprints/Actors/Buidings/BP_PlacedBuilding.BP_PlacedBuilding_C" (`self.GetTransform` (`self.PlaceableActor`)) "AlwaysSpawn" "OverrideRootScale" null null))
              (set `/Game/CityBuilder/Core/Blueprints/Actors/Buidings/BP_PlacedBuilding.BuildingToSpawn` (select `/Game/CityBuilder/Core/Data/Enums/E_BuildingTypes` (`self.PlaceableBuildingType`) :`NewEnumerator0` "/Game/CityBuilder/Core/Blueprints/Actors/Buidings/BP_Building_House.BP_Building_House_C" :`NewEnumerator1` "/Game/CityBuilder/Core/Blueprints/Actors/Buidings/BP_Building_Mine.BP_Building_Mine_C" :`NewEnumerator2` "/Game/CityBuilder/Core/Blueprints/Actors/Buidings/BP_Building_Farm.BP_Building_Farm_C" :`NewEnumerator3` "/Game/CityBuilder/Core/Blueprints/Actors/Buidings/BP_Building_Dock.BP_Building_Dock_C" :`NewEnumerator4` "/Game/CityBuilder/Core/Blueprints/Actors/Buidings/BP_Building_Lumbermill.BP_Building_Lumbermill_C" :`NewEnumerator5` "/Game/CityBuilder/Core/Blueprints/Actors/Buidings/BP_Building_Church.BP_Building_Church_C" :`NewEnumerator6` "/Game/CityBuilder/Core/Blueprints/Actors/Buidings/BP_Building_Market.BP_Building_Market_C" :`NewEnumerator7` "/Game/CityBuilder/Core/Blueprints/Actors/Buidings/BP_Building_Blacksmith.BP_Building_Blacksmith_C" :`NewEnumerator8` "/Game/CityBuilder/Core/Blueprints/Actors/Buidings/BP_Building_Tailor.BP_Building_Tailor_C" :`NewEnumerator9` "/Game/CityBuilder/Core/Blueprints/Actors/Buidings/BP_Building_Tavern.BP_Building_Tavern_C" :`NewEnumerator10` "/Game/CityBuilder/Core/Blueprints/Actors/Buidings/BP_Building_TownHall.BP_Building_TownHall_C" :`NewEnumerator11` "/Game/CityBuilder/Core/Blueprints/Actors/Buidings/BP_Building_HuntingCabin.BP_Building_HuntingCabin_C" :`NewEnumerator12` "/Game/CityBuilder/Core/Blueprints/Actors/Buidings/BP_Building_Pasture.BP_Building_Pasture_C" :`NewEnumerator13` "/Game/CityBuilder/Core/Blueprints/Actors/Buidings/BP_Building_SchoolHouse.BP_Building_SchoolHouse_C" :`NewEnumerator14` "/Game/CityBuilder/Core/Blueprints/Actors/Buidings/BP_Building_IronMine.BP_Building_IronMine_C" :`NewEnumerator15` "/Game/CityBuilder/Core/Blueprints/Actors/Buidings/BP_Building_HouseT2.BP_Building_HouseT2_C" :`NewEnumerator16` "/Game/CityBuilder/Core/Blueprints/Actors/Buidings/BP_Building_Library.BP_Building_Library_C" :`NewEnumerator17` "/Game/CityBuilder/Core/Blueprints/Actors/Buidings/BP_Building_Workshop.BP_Building_Workshop_C" :`NewEnumerator18` "/Game/CityBuilder/Core/Blueprints/Actors/Buidings/BP_Building_TradingPost.BP_Building_TradingPost_C" :`NewEnumerator19` "/Game/CityBuilder/Core/Blueprints/Actors/Buidings/BP_Building_Carpenter.BP_Building_Carpenter_C" :!type "Actor Class Reference") _returnvalue_2)
              (set `/Game/CityBuilder/Core/Blueprints/Actors/Buidings/BP_PlacedBuilding.BuildingMesh` (`self.BuildingMesh`) _returnvalue_2)
              (bind _returnvalue_3 (`|GetDataTableRow` "/Game/CityBuilder/Core/Data/DataTables/DT_BuildingsData.DT_BuildingsData" (select `/Game/CityBuilder/Core/Data/Enums/E_BuildingTypes` (`self.PlaceableBuildingType`) :`NewEnumerator0` "1" :`NewEnumerator1` "2" :`NewEnumerator2` "3" :`NewEnumerator3` "4" :`NewEnumerator4` "5" :`NewEnumerator5` "6" :`NewEnumerator6` "7" :`NewEnumerator7` "8" :`NewEnumerator8` "9" :`NewEnumerator9` "10" :`NewEnumerator10` "11" :`NewEnumerator11` "12" :`NewEnumerator12` "13" :`NewEnumerator13` "14" :`NewEnumerator14` "15" :`NewEnumerator15` "16" :`NewEnumerator16` "17" :`NewEnumerator17` "18" :`NewEnumerator18` "19" :`NewEnumerator19` "20" :!type "Name"))
                (:`then`
                  (set `/Game/CityBuilder/Core/Blueprints/GS_CityBuilderGameState.PopulationBalance` (- (`/Game/CityBuilder/Core/Blueprints/GS_CityBuilderGameState.PopulationBalance` _gamestate) (`.PopulationValue_3_648D732E414F3713957352ACD408C8A8` (break `/Game/CityBuilder/Core/Data/Structs/ST_BuildingPrices` _returnvalue_3))) _gamestate_2)
                  (set `/Game/CityBuilder/Core/Blueprints/GS_CityBuilderGameState.ResearchBalance` (- (`/Game/CityBuilder/Core/Blueprints/GS_CityBuilderGameState.ResearchBalance` _gamestate) (`.ResearchValue_5_FCF0E4F44047BE255D8BC08166812A03` (break `/Game/CityBuilder/Core/Data/Structs/ST_BuildingPrices` _returnvalue_3))) _gamestate_2)
                  (set `/Game/CityBuilder/Core/Blueprints/GS_CityBuilderGameState.ProductionBalance` (- (`/Game/CityBuilder/Core/Blueprints/GS_CityBuilderGameState.ProductionBalance` _gamestate) (`.ProductionValue_12_4CDC79E64588D40273901C9B60FBA17A` (break `/Game/CityBuilder/Core/Data/Structs/ST_BuildingPrices` _returnvalue_3))) _gamestate_2)
                  (set `/Game/CityBuilder/Core/Blueprints/GS_CityBuilderGameState.PopulationMax` (+ (`.PopulationMaxIncrease_25_B31463134965716354B917AB80EBDC3E` (break `/Game/CityBuilder/Core/Data/Structs/ST_BuildingPrices` _returnvalue_3)) (`/Game/CityBuilder/Core/Blueprints/GS_CityBuilderGameState.PopulationMax` _gamestate_2)) _gamestate_2)
                  (set `/Game/CityBuilder/Core/Blueprints/GS_CityBuilderGameState.ResearchMax` (+ (`.ResearchMaxIncrease_26_754C4BCB4CF13F5F5D6041AFC6CF3156` (break `/Game/CityBuilder/Core/Data/Structs/ST_BuildingPrices` _returnvalue_3)) (`/Game/CityBuilder/Core/Blueprints/GS_CityBuilderGameState.ResearchMax` _gamestate_2)) _gamestate_2)
                  (set `/Game/CityBuilder/Core/Blueprints/GS_CityBuilderGameState.ProductionMax` (+ (`.ProductionMaxIncrease_27_4A5C7F404CAD3F530588789CD9CBFF77` (break `/Game/CityBuilder/Core/Data/Structs/ST_BuildingPrices` _returnvalue_3)) (`/Game/CityBuilder/Core/Blueprints/GS_CityBuilderGameState.ProductionMax` _gamestate_2)) _gamestate_2)
                  (set `/Game/CityBuilder/Core/Blueprints/GS_CityBuilderGameState.HappinessPercent` (+ (`.HappinessIncrease_33_92E8F9E5475FC5A00080F29CD4F776B5` (break `/Game/CityBuilder/Core/Data/Structs/ST_BuildingPrices` _returnvalue_3)) (`/Game/CityBuilder/Core/Blueprints/GS_CityBuilderGameState.HappinessPercent` _gamestate_2)) _gamestate_2)
                  (bind _output_get (set `self.BuildingMesh` (`self.GetBuildingMesh`)))
                  (bind _asbp_dummy_building (cast `/Game/CityBuilder/Core/Blueprints/Actors/Buidings/BP_DummyBuilding` (`self.PlaceableActor`))
                    (:`then`
                      (`StaticMeshComponent.SetStaticMesh` (`/Game/CityBuilder/Core/Blueprints/Actors/Buidings/BP_DummyBuilding.BuidingMesh` _asbp_dummy_building) _output_get))
                    (:`CastFailed`
                      _))
                  (bind _output_2 (`self.CanAfford?`)
                    (:`true`
                      (set `/Game/CityBuilder/Core/Blueprints/Components/BPC_PlaceableComp.bCanAfford?` _output_2 (`self.GetComponentByClass` (`self.PlaceableActor`) "/Game/CityBuilder/Core/Blueprints/Components/BPC_PlaceableComp.BPC_PlaceableComp_C"))
                      (`self.SetPlacementModeEnabled` false))))))))))))

(fn `SpawnCheckTraces`
  (params (MainHitLocation :type "Vector Structure"))
  (returns (`bValidLocation?` :type Boolean))
  (bind _tracelocation (`self.TraceLocation`))
  (bind _returnvalue (* _tracelocation -1.0))
  (for _index (range 4)
    (bind _returnvalue_2 (+ MainHitLocation (`KismetMathLibrary.MakeVector` (select `int` _index :`0` _returnvalue :`1` _tracelocation :`2` _tracelocation :`3` _returnvalue) (select `int` _index :`0` _tracelocation :`1` _tracelocation :`2` _returnvalue :`3` _returnvalue) 25.0)))
    (bind _outhit (`KismetSystemLibrary.LineTraceSingle` :`Start` _returnvalue_2 :`End` (- _returnvalue_2 (0.0 0.0 35.0)) :`TraceChannel` "TraceTypeQuery3" :`TraceColor` (struct :`R` 0.848742 :`B` 1.0 :`A` 1.0) :`TraceHitColor` (struct :`R` 1.0 :`G` 0.861242 :`A` 1.0)))
    (bind (_bblockinghit _binitialoverlap _time _distance) (`GameplayStatics.BreakHitResult` _outhit))
    (if (and _bblockinghit (> _distance 10.0))
      (bind _returnvalue_3 (== _index 3))
      (if _returnvalue_3
        (return _returnvalue_3))
      (else
        (break)))))

(fn `SpawnStartingActors`
  (bind _returnvalue (`KismetMathLibrary.RandomFloatInRange` -4000.0 4000.0))
  (bind _returnvalue_2 (`KismetMathLibrary.RandomFloatInRange` -4000.0 4000.0))
  (bind _returnvalue_3 (mod _returnvalue_2 250.0))
  (bind _returnvalue_4 (mod _returnvalue 250.0))
  (bind _returnvalue_5 (- _returnvalue_2 _returnvalue_3))
  (bind _returnvalue_6 (- _returnvalue _returnvalue_4))
  (bind _returnvalue_7 (select `bool` (< _returnvalue_3 125.0) :`false` _returnvalue_5 :`true` (+ _returnvalue_5 250.0)))
  (bind _returnvalue_8 (select `bool` (< _returnvalue_4 125.0) :`false` _returnvalue_6 :`true` (+ _returnvalue_6 250.0)))
  (for _ (range 101)
    (bind _outhit (`KismetSystemLibrary.LineTraceSingle` :`Start` (`KismetMathLibrary.MakeVector` _returnvalue_8 _returnvalue_7 5000.0) :`End` (`KismetMathLibrary.MakeVector` _returnvalue_8 _returnvalue_7) :`TraceChannel` "TraceTypeQuery3" :`TraceColor` (struct :`G` 0.197584 :`B` 1.0 :`A` 1.0)))
    (bind (_bblockinghit _binitialoverlap _time _distance _location _impactpoint _normal _impactnormal _physmat _hitactor _hitcomponent) (`GameplayStatics.BreakHitResult` _outhit))
    (if (and _bblockinghit (not (`ActorComponent.ComponentHasTag` _hitcomponent "Water")))
      (bind _bvalidlocation_ (`self.SpawnCheckTraces` _location))
      (if _bvalidlocation_
        (`|ExecutionSequence`
          (:`then_0`
            (break))
          (:`then_1`
            (`|SpawnActorFromClass` "/Game/CityBuilder/Core/Blueprints/Actors/Buidings/BP_Building_TownCenter.BP_Building_TownCenter_C" (`KismetMathLibrary.MakeTransform` _location (`KismetMathLibrary.MakeRotator` 0.0 0.0 (`KismetMathLibrary.RandomFloatInRange` 0.0 360.0))) "AlwaysSpawn" "OverrideRootScale" null null)
            (`self.K2_SetActorLocation` (`GameplayStatics.GetPlayerPawn` 0) (+ _location (0.0 0.0 100.0)) false false)))))))

(fn `UpdatePlacement`
  (bind (_worldlocation _worlddirection) (`self.DeprojectMousePositionToWorld`))
  (bind _outhit (`KismetSystemLibrary.LineTraceSingle` _worldlocation (+ _worldlocation (* _worlddirection 25000.0)) "TraceTypeQuery3"))
  (bind (_bblockinghit _binitialoverlap _time _distance _location _impactpoint _normal _impactnormal) (`GameplayStatics.BreakHitResult` _outhit))
  (if _bblockinghit
    (`KismetSystemLibrary.PrintString` (`KismetStringLibrary.Conv_VectorToString` _impactnormal) true false (struct :`G` 0.66 :`B` 1.0 :`A` 1.0) 1.0)
    (`self.K2_SetActorLocation` (`self.PlaceableActor`) _location false false)
    (`self.CanAfford?`)))

(fn `UserConstructionScript`)