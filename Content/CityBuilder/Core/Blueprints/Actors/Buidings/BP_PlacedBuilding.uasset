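; BP_PlacedBuilding is a temporary construction-stage actor that shows build progress, then replaces itself with the real building.
; On BeginPlay it removes its selectable component and runs a timeline that drives a circular progress bar widget's material.
; When the timeline finishes, it spawns BuildingToSpawn at its transform, passes on the mesh and buff multiplier, and destroys itself.
; The timeline play rate is fixed, leaving ConstructionTime unused.
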(event `self.ReceiveBeginPlay`
  (`ActorComponent.K2_DestroyComponent` (`self.BP_Selectable_Building`))
  (bind _returnvalue (`AddComponent|NODE_AddWidgetComponent-0`))
  (bind _aswbp_circular_progress_bar (cast `/Game/CityBuilder/UI/Blueprints/InWorld/WBP_CircularProgressBar` (`WidgetComponent.GetWidget` _returnvalue)))
  (`TimelineComponent.SetPlayRate` (`self.ConstructionTimeline`) (/ 1.0 1.0))
  (`KismetSystemLibrary.Delay` 0.1)
  (bind (_direction _alpha) (`Timeline|ConstructionTimeline` :!via `PlayFromStart`)
    (:`Update`
      (`MaterialInstanceDynamic.SetScalarParameterValue` (`/Game/CityBuilder/UI/Blueprints/InWorld/WBP_CircularProgressBar.ProgressBarMat` _aswbp_circular_progress_bar) "Alpha" _alpha))
    (:`Finished`
      (`ActorComponent.K2_DestroyComponent` _returnvalue)
      (bind _returnvalue_2 (`|SpawnActorFromClass` (`self.BuildingToSpawn`) (`self.GetTransform`) "AlwaysSpawn" "OverrideRootScale" null null))
      (bind _asbp_building_base (cast `/Game/CityBuilder/Core/Blueprints/Actors/Buidings/BP_Building_Base` _returnvalue_2))
      (`StaticMeshComponent.SetStaticMesh` (`/Game/CityBuilder/Core/Blueprints/BP_InWorld_Base.BaseMesh` _asbp_building_base) (`self.BuildingMesh`))
      (set `/Game/CityBuilder/Core/Blueprints/BP_InWorld_Base.BuffMultiplier` (`self.BuffMultiplier`) _asbp_building_base)
      (`self.K2_DestroyActor`))))

(fn `UserConstructionScript`)