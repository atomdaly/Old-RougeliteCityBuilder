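; Base actor for city-builder buildings that registers a building's economic effect when it begins play.
; BeginPlay labels it with its type, passes that type to its BPSelectableBuilding, and starts the progress bar.
; Its DT_BuildingsData row, selected by type, immediately adds population, research, production and happiness increases to GameState's change rates.
; A timeline scaled by CurrentTime drives the circular progress material in the first WBP_SelectedBuildingMenu found.
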(event `self.ReceiveBeginPlay`
  (bind _gamestate (`self.GameState`))
  (`parent.ReceiveBeginPlay`)
  (`TextRenderComponent.K2_SetText` (`self.TextRender`) (`KismetTextLibrary.Conv_StringToText` (`|GetEnumeratorNameAsString` (`self.BuildingType`))))
  (set `/Game/CityBuilder/Core/Blueprints/Components/SelectableComps/BP_Selectable_Building.BuildingType` (`self.BuildingType`) (`self.BP_Selectable_Building`))
  (`self.ProgressBar`)
  (bind _returnvalue (`|GetDataTableRow` "/Game/CityBuilder/Core/Data/DataTables/DT_BuildingsData.DT_BuildingsData" (select `/Game/CityBuilder/Core/Data/Enums/E_BuildingTypes` (`self.BuildingType`) :`NewEnumerator0` "1" :`NewEnumerator1` "2" :`NewEnumerator2` "3" :`NewEnumerator3` "4" :`NewEnumerator4` "5" :`NewEnumerator5` "6" :`NewEnumerator6` "7" :`NewEnumerator7` "8" :`NewEnumerator8` "9" :`NewEnumerator9` "10" :`NewEnumerator10` "11" :`NewEnumerator11` "12" :`NewEnumerator12` "13" :`NewEnumerator13` "14" :`NewEnumerator14` "15" :`NewEnumerator15` "16" :`NewEnumerator16` "17" :`NewEnumerator17` "18" :`NewEnumerator18` "19" :`NewEnumerator19` "20" :`NewEnumerator20` "21" :!type "Name"))
    (:`then`
      (`|ExecutionSequence`
        (:`then_0`
          (set `/Game/CityBuilder/Core/Blueprints/GS_CityBuilderGameState.PopulationChange` (+ (`/Game/CityBuilder/Core/Blueprints/GS_CityBuilderGameState.PopulationChange` _gamestate) (`.PopulationIncrease_19_DCE2DDC744B3F565A3F7078B7619E73D` (break `/Game/CityBuilder/Core/Data/Structs/ST_BuildingPrices` _returnvalue))) _gamestate))
        (:`then_1`
          (set `/Game/CityBuilder/Core/Blueprints/GS_CityBuilderGameState.ResearchChange` (+ (`/Game/CityBuilder/Core/Blueprints/GS_CityBuilderGameState.ResearchChange` _gamestate) (`.ResearchIncrease_20_1A94CEF1416BDBF1FF39258DD977BC8A` (break `/Game/CityBuilder/Core/Data/Structs/ST_BuildingPrices` _returnvalue))) _gamestate))
        (:`then_2`
          (set `/Game/CityBuilder/Core/Blueprints/GS_CityBuilderGameState.ProductionChange` (+ (`/Game/CityBuilder/Core/Blueprints/GS_CityBuilderGameState.ProductionChange` _gamestate) (`.ProductionIncrease_21_6C447CE543E6D27DC8EA1C95A38E9F2E` (break `/Game/CityBuilder/Core/Data/Structs/ST_BuildingPrices` _returnvalue))) _gamestate))
        (:`then_3`
          (set `/Game/CityBuilder/Core/Blueprints/GS_CityBuilderGameState.HappinessChange` (+ (`/Game/CityBuilder/Core/Blueprints/GS_CityBuilderGameState.HappinessChange` _gamestate) (`.HappinessIncrease_33_92E8F9E5475FC5A00080F29CD4F776B5` (break `/Game/CityBuilder/Core/Data/Structs/ST_BuildingPrices` _returnvalue))) _gamestate))))))

(event `ProgressBar`
  (bind _foundwidgets (`WidgetBlueprintLibrary.GetAllWidgetsOfClass` "/Game/CityBuilder/UI/Blueprints/HUD/WBP_SelectedBuildingMenu.WBP_SelectedBuildingMenu_C" false))
  (bind _output (`|GetArrayItem` _foundwidgets))
  (`/Engine/EditorBlueprintResources/StandardMacros.IsValid` _output
    (:`Is Valid`
      (`TimelineComponent.SetPlayRate` (`self.ProgressBarTimeline`) (/ 1.0 (`self.CurrentTime`)))
      (bind (_direction _alpha) (`Timeline|ProgressBarTimeline` :!via `PlayFromStart`)
        (:`Update`
          (`MaterialInstanceDynamic.SetScalarParameterValue` (`/Game/CityBuilder/UI/Blueprints/InWorld/WBP_CircularProgressBar.ProgressBarMat` (`/Game/CityBuilder/UI/Blueprints/HUD/WBP_SelectedBuildingMenu.WBP_CircularProgressBar` _output)) "Alpha" _alpha))))))

(fn `UserConstructionScript`)