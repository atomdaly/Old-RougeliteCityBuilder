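; Decoration actor that hangs bunting between a start and end point in the city builder.
; On BeginPlay it rebuilds the spline from both endpoints plus a midpoint dropped by a random amount to create sag.
; SetSplineMesh then adds a spline mesh component per segment, matching tangents and point scales; the construction script runs the same function on the existing spline.
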(event `self.ReceiveBeginPlay`
  (bind _splinepathend (`self.SplinePathEnd`))
  (bind _spline (`self.Spline`))
  (bind _splinepathstart (`self.SplinePathStart`))
  (`SplineComponent.ClearSplinePoints` _spline true)
  (`SplineComponent.AddSplinePoint` _spline _splinepathstart "World" true)
  (`SplineComponent.AddSplinePointAtIndex` _spline (+ (/ (+ _splinepathstart _splinepathend) 2.0) (`KismetMathLibrary.MakeVector` 0.0 0.0 (`KismetMathLibrary.RandomFloatInRange` -25.0 -100.0))) 1 "World" true)
  (`SplineComponent.AddSplinePoint` _spline _splinepathend "World" true)
  (`self.SetSplineMesh`))

(fn `SetSplineMesh`
  (bind _spline (`self.Spline`))
  (for _index (range (+ (- (`SplineComponent.GetNumberOfSplinePoints` (`self.Spline`)) 2) 1))
    (bind _returnvalue (`AddComponent|NODE_AddSplineMeshComponent-0`))
    (`SplineMeshComponent.SetForwardAxis` _returnvalue "X" true)
    (bind _returnvalue_2 (+ _index 1))
    (`SplineMeshComponent.SetStartAndEnd` _returnvalue (`SplineComponent.GetLocationAtSplinePoint` _spline _index "Local") (`SplineComponent.GetTangentAtSplinePoint` _spline _index "Local") (`SplineComponent.GetLocationAtSplinePoint` _spline _returnvalue_2 "Local") (`SplineComponent.GetTangentAtSplinePoint` _spline _returnvalue_2 "Local") true)
    (bind (_returnvalue_x _returnvalue_y _returnvalue_z) (`KismetMathLibrary.BreakVector` (`SplineComponent.GetScaleAtSplinePoint` _spline _index)))
    (`SplineMeshComponent.SetStartScale` _returnvalue (`KismetMathLibrary.MakeVector2D` _returnvalue_y _returnvalue_z) true)
    (bind (_returnvalue_x_2 _returnvalue_y_2 _returnvalue_z_2) (`KismetMathLibrary.BreakVector` (`SplineComponent.GetScaleAtSplinePoint` _spline _returnvalue_2)))
    (`SplineMeshComponent.SetEndScale` _returnvalue (`KismetMathLibrary.MakeVector2D` _returnvalue_y_2 _returnvalue_z_2) true)))

(fn `UserConstructionScript`
  (`self.SetSplineMesh`))