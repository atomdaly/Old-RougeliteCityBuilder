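; BP_PathGenerator is a city-builder decoration actor that builds a gently curved path between a start and an end location.
; On BeginPlay it rebuilds its spline as three raised points, pushing the midpoint randomly sideways in proportion to path length.
; SetSplineMesh, also run at construction, adds a spline mesh per segment.
; It then spawns a BP_PathPoint at the middle point, plus a randomly rotated BP_Lampost on long paths.
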(event `self.ReceiveBeginPlay`
  (bind _spline (`self.Spline`))
  (bind _returnvalue (`SplineComponent.GetLocationAtSplinePoint` _spline 1 "Local"))
  (bind _returnvalue_2 (+ (`self.SplinePathEnd`) (0.0 0.0 100.0)))
  (bind _returnvalue_3 (+ (`self.SplinePathStart`) (0.0 0.0 100.0)))
  (bind _returnvalue_4 (/ (`KismetMathLibrary.VSize` (- _returnvalue_3 _returnvalue_2)) 10.0))
  (`SplineComponent.ClearSplinePoints` _spline true)
  (`SplineComponent.AddSplinePoint` _spline _returnvalue_3 "World" true)
  (`SplineComponent.AddSplinePointAtIndex` _spline (+ (/ (+ _returnvalue_3 _returnvalue_2) 2.0) (* (`KismetMathLibrary.GetRightVector` (`KismetMathLibrary.FindLookAtRotation` _returnvalue_3 _returnvalue_2)) (`KismetMathLibrary.RandomFloatInRange` (* _returnvalue_4 -1.0) _returnvalue_4))) 1 "World" true)
  (`SplineComponent.AddSplinePoint` _spline _returnvalue_2 "World" true)
  (`self.SetSplineMesh`)
  (`|SpawnActorFromClass` "/Game/CityBuilder/Core/Blueprints/Actors/Decoration/BP_PathPoint.BP_PathPoint_C" (`KismetMathLibrary.MakeTransform` _returnvalue) "Undefined" "OverrideRootScale" null null)
  (if (>= (`SplineComponent.GetSplineLength` _spline) 2000.0)
    (`|SpawnActorFromClass` "/Game/CityBuilder/Core/Blueprints/Actors/Decoration/BP_Lampost.BP_Lampost_C" (`KismetMathLibrary.MakeTransform` _returnvalue (`KismetMathLibrary.MakeRotator` 0.0 0.0 (`KismetMathLibrary.RandomFloatInRange` 0.0 360.0))) "Undefined" "OverrideRootScale" null null)))

(fn `SetSplineMesh`
  (bind _spline (`self.Spline`))
  (for _index (range (+ (- (`SplineComponent.GetNumberOfSplinePoints` (`self.Spline`)) 2) 1))
    (bind _returnvalue (`AddComponent|NODE_AddSplineMeshComponent-0`))
    (`SplineMeshComponent.SetForwardAxis` _returnvalue "X" true)
    (bind _returnvalue_2 (+ _index 1))
    (`SplineMeshComponent.SetStartAndEnd` _returnvalue (`SplineComponent.GetLocationAtSplinePoint` _spline _index "Local") (`SplineComponent.GetTangentAtSplinePoint` _spline _index "Local") (`SplineComponent.GetLocationAtSplinePoint` _spline _returnvalue_2 "Local") (`SplineComponent.GetTangentAtSplinePoint` _spline _returnvalue_2 "Local") true)
    (bind (_returnvalue_x _returnvalue_y _returnvalue_z) (`KismetMathLibrary.BreakVector` (`SplineComponent.GetScaleAtSplinePoint` _spline _index)))
    (`SplineMeshComponent.SetStartScale` _returnvalue (`KismetMathLibrary.MakeVector2D` _returnvalue_y _returnvalue_z) true)
    (bind (_returnvalue_x_2 _returnvalue_y_2 _returnvalue_z_2) (`KismetMathLibrary.BreakVector` (`SplineComponent.GetScaleAtSplinePoint` _spline _returnvalue_2)))
    (`SplineMeshComponent.SetEndScale` _returnvalue (`KismetMathLibrary.MakeVector2D` _returnvalue_y_2 _returnvalue_z_2) true)))

(fn `UserConstructionScript`
  (`self.SetSplineMesh`))