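; Base resource actor for the city builder that turns one population into one production when its widget button is clicked.
; A click requires production not at its maximum and at least two population, then locks the button and starts a five-second harvest timer.
; A temporary widget component shows a circular progress bar, driven by a timeline through a material parameter.
; The timer adds the production to GameState and unlocks the button.
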(event `self.ReceiveBeginPlay`
  (`parent.ReceiveBeginPlay`))

(event `self.WidgetButtonClicked`
  (bind _gamestate (`self.GameState`))
  (bind _populationbalance (`/Game/CityBuilder/Core/Blueprints/GS_CityBuilderGameState.PopulationBalance` _gamestate))
  (if (and (!= (`/Game/CityBuilder/Core/Blueprints/GS_CityBuilderGameState.ProductionMax` _gamestate) (`/Game/CityBuilder/Core/Blueprints/GS_CityBuilderGameState.ProductionBalance` _gamestate)) (>= _populationbalance 2))
    (set `/Game/CityBuilder/Core/Blueprints/GS_CityBuilderGameState.PopulationBalance` (- _populationbalance 1) _gamestate)
    (set `self.bCanPressWidgetButton?` false)
    (`KismetSystemLibrary.K2_SetTimerDelegate` (delegate `HarvestResource`) 5.0)
    (bind _returnvalue (`AddComponent|NODE_AddWidgetComponent-0`))
    (bind _aswbp_circular_progress_bar (cast `/Game/CityBuilder/UI/Blueprints/InWorld/WBP_CircularProgressBar` (`WidgetComponent.GetWidget` _returnvalue)))
    (`KismetSystemLibrary.Delay` 0.1)
    (bind (_direction _alpha) (`Timeline|ProgressBarTimeline` :!via `PlayFromStart`)
      (:`Update`
        (`MaterialInstanceDynamic.SetScalarParameterValue` (`/Game/CityBuilder/UI/Blueprints/InWorld/WBP_CircularProgressBar.ProgressBarMat` _aswbp_circular_progress_bar) "Alpha" _alpha))
      (:`Finished`
        (`ActorComponent.K2_DestroyComponent` _returnvalue)))))

(event `HarvestResource`
  (bind _gamestate (`self.GameState`))
  (set `/Game/CityBuilder/Core/Blueprints/GS_CityBuilderGameState.ProductionBalance` (+ (`/Game/CityBuilder/Core/Blueprints/GS_CityBuilderGameState.ProductionBalance` _gamestate) 1) _gamestate)
  (set `self.bCanPressWidgetButton?` true))

(fn `UserConstructionScript`)