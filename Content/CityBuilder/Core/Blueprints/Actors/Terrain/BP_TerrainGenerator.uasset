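; City builder terrain generator actor that builds a random blocky tile terrain when play begins.
; RandomlyGenerateTerrain rolls two frequencies and two heights, then fills a square grid of BaseMesh instances.
; Each tile's height sums two layered products of sine waves, rounded to tile-size steps for a terraced look.
; GenerateTerrain is a near-identical variant using the current parameters without randomizing, and is not called here.
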(event `self.ReceiveBeginPlay`
  (`self.RandomlyGenerateTerrain`))

(fn `GenerateTerrain`
  (bind _terrainsize (`self.TerrainSize`))
  (bind _tilesize (`self.TileSize`))
  (bind _frequency_2 (`self.Frequency_2`))
  (bind _frequency_1 (`self.Frequency_1`))
  (`InstancedStaticMeshComponent.ClearInstances` (`self.BaseMesh`))
  (for _index (range (+ _terrainsize 1))
    (for _index_2 (range (+ _terrainsize 1))
      (`InstancedStaticMeshComponent.AddInstance` (`self.BaseMesh`) (`KismetMathLibrary.Conv_VectorToTransform` (`KismetMathLibrary.MakeVector` (`KismetMathLibrary.Conv_IntToDouble` (* _index _tilesize)) (`KismetMathLibrary.Conv_IntToDouble` (* _index_2 _tilesize)) (`KismetMathLibrary.Conv_IntToDouble` (* _tilesize (`KismetMathLibrary.Round` (+ (* (`KismetMathLibrary.DegSin` (* _index _frequency_1)) (`KismetMathLibrary.DegSin` (* (* _index_2 _frequency_1) 0.4)) (`self.Height_1`)) (* (`KismetMathLibrary.DegSin` (* (* _index _frequency_2) 0.7)) (`KismetMathLibrary.DegSin` (* _index_2 _frequency_2)) (`self.Height_2`))))))))))))

(fn `RandomlyGenerateTerrain`
  (bind _terrainsize (`self.TerrainSize`))
  (bind _tilesize (`self.TileSize`))
  (bind _frequency_1 (`self.Frequency_1`))
  (bind _frequency_2 (`self.Frequency_2`))
  (`InstancedStaticMeshComponent.ClearInstances` (`self.BaseMesh`))
  (set `self.Frequency_1` (`KismetMathLibrary.RandomFloatInRange` 2.5 5.0))
  (set `self.Frequency_2` (`KismetMathLibrary.RandomFloatInRange` 10.0 15.0))
  (set `self.Height_1` (`KismetMathLibrary.RandomFloatInRange` 0.0 0.75))
  (set `self.Height_2` (`KismetMathLibrary.RandomFloatInRange` 1.0 2.5))
  (for _index (range 1 (+ _terrainsize 1))
    (for _index_2 (range 1 (+ _terrainsize 1))
      (`InstancedStaticMeshComponent.AddInstance` (`self.BaseMesh`) (`KismetMathLibrary.Conv_VectorToTransform` (`KismetMathLibrary.MakeVector` (`KismetMathLibrary.Conv_IntToDouble` (* _index _tilesize)) (`KismetMathLibrary.Conv_IntToDouble` (* _index_2 _tilesize)) (`KismetMathLibrary.Conv_IntToDouble` (* _tilesize (`KismetMathLibrary.Round` (+ (* (`KismetMathLibrary.DegSin` (* _index _frequency_1)) (`KismetMathLibrary.DegSin` (* (* _index_2 _frequency_1) 0.2)) (`self.Height_1`)) (* (`KismetMathLibrary.DegSin` (* (* _index _frequency_2) 0.7)) (`KismetMathLibrary.DegSin` (* _index_2 _frequency_2)) (`self.Height_2`))))))))))))

(fn `UserConstructionScript`)