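; Selectable component for city-builder resources such as stone and wood, handling what happens when one is selected or deselected.
; On BeginPlay it runs the parent logic, then derives the display name from its resource type.
; Selection fills the HUD's resource menu with name, description and owning actor, enables custom depth on the mesh and opens the menu.
; Deselection clears that actor, disables custom depth and closes the menu.
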(event `self.ReceiveBeginPlay`
  (`parent.ReceiveBeginPlay`)
  (set `self.ResourceName` (select `/Game/CityBuilder/Core/Data/Enums/E_ResourceTypes` (`self.ResourceType`) :`NewEnumerator0` "Stone" :`NewEnumerator1` "Wood" :!type "Text")))

(event `self.Selected`
  (bind _hudref (`self.HUDRef`))
  (bind _wbp_selectedresourcemenu (`/Game/CityBuilder/UI/Blueprints/HUD/WBP_HUD.WBP_SelectedResourceMenu` _hudref))
  (set `self.bIsClicked?` true)
  (`TextBlock.SetText` (`/Game/CityBuilder/UI/Blueprints/HUD/WBP_SelectedResourceMenu.ObjectName` _wbp_selectedresourcemenu) (`self.ResourceName`))
  (`RichTextBlock.SetText` (`/Game/CityBuilder/UI/Blueprints/HUD/WBP_SelectedResourceMenu.ObjectDescription` _wbp_selectedresourcemenu) (`self.ResourceDescription`))
  (set `/Game/CityBuilder/UI/Blueprints/HUD/WBP_SelectedResourceMenu.SelectedActor` (`self.OwningActor`) _wbp_selectedresourcemenu)
  (`PrimitiveComponent.SetRenderCustomDepth` (`self.MeshRef`) true)
  (`/Game/CityBuilder/UI/Blueprints/HUD/WBP_HUD.OpenSelectedResourceMenu` _hudref))

(event `self.Deselected`
  (bind _hudref (`self.HUDRef`))
  (set `self.bIsClicked?` false)
  (set `/Game/CityBuilder/UI/Blueprints/HUD/WBP_SelectedResourceMenu.SelectedActor` null (`/Game/CityBuilder/UI/Blueprints/HUD/WBP_HUD.WBP_SelectedResourceMenu` _hudref))
  (`PrimitiveComponent.SetRenderCustomDepth` (`self.MeshRef`) false)
  (`/Game/CityBuilder/UI/Blueprints/HUD/WBP_HUD.CloseSelectedResourceMenu` _hudref))