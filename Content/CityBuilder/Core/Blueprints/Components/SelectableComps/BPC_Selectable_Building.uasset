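; Selectable component for city-builder buildings that handles selection highlighting and the selected-building menu.
; After a short delay on BeginPlay, it maps BuildingType to a display name and prints it.
; Selection fills the HUD menu with name, description and owning actor, opens it, and enables the mesh's custom depth rendering.
; Deselection clears the menu's actor, closes it and disables custom depth.
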(event `self.ReceiveBeginPlay`
  (`parent.ReceiveBeginPlay`)
  (`KismetSystemLibrary.Delay` 0.1)
  (bind _output_get (set `self.BuildingName` (select `/Game/CityBuilder/Core/Data/Enums/E_BuildingTypes` (`self.BuildingType`) :`NewEnumerator0` "House" :`NewEnumerator1` "Mine" :`NewEnumerator2` "Farm" :`NewEnumerator3` "Dock" :`NewEnumerator4` "LumberMill" :`NewEnumerator5` "Church" :`NewEnumerator6` "Market" :`NewEnumerator7` "Blacksmith" :`NewEnumerator8` "Tailor" :`NewEnumerator9` "Tavern" :`NewEnumerator10` "TownHall" :`NewEnumerator11` "HuntingCabin" :`NewEnumerator12` "Pasture" :`NewEnumerator13` "SchoolHouse" :`NewEnumerator14` "IronMine" :`NewEnumerator15` "HouseT2" :`NewEnumerator16` "Library" :`NewEnumerator17` "Workshop" :`NewEnumerator18` "TradingPost" :`NewEnumerator19` "Carpenter" :`NewEnumerator20` "TownCenter" :!type "Text")))
  (`KismetSystemLibrary.PrintString` (`KismetTextLibrary.Conv_TextToString` _output_get) true false (struct :`R` 0.745404 :`G` 0.008023 :`B` 0.107023 :`A` 1.0)))

(event `self.Selected`
  (bind _hudref (`self.HUDRef`))
  (bind _wbp_selectedbuildingmenu (`/Game/CityBuilder/UI/Blueprints/HUD/WBP_HUD.WBP_SelectedBuildingMenu` _hudref))
  (set `self.bIsClicked?` true)
  (`TextBlock.SetText` (`/Game/CityBuilder/UI/Blueprints/HUD/WBP_SelectedBuildingMenu.ObjectName` _wbp_selectedbuildingmenu) (`self.BuildingName`))
  (`RichTextBlock.SetText` (`/Game/CityBuilder/UI/Blueprints/HUD/WBP_SelectedBuildingMenu.ObjectDescription` _wbp_selectedbuildingmenu) (`self.BuildingDescription`))
  (set `/Game/CityBuilder/UI/Blueprints/HUD/WBP_SelectedBuildingMenu.SelectedActor` (`self.OwningActor`) _wbp_selectedbuildingmenu)
  (`PrimitiveComponent.SetRenderCustomDepth` (`self.MeshRef`) true)
  (`/Game/CityBuilder/UI/Blueprints/HUD/WBP_HUD.OpenSelectedBuildingMenu` _hudref))

(event `self.Deselected`
  (bind _hudref (`self.HUDRef`))
  (set `self.bIsClicked?` false)
  (set `/Game/CityBuilder/UI/Blueprints/HUD/WBP_SelectedBuildingMenu.SelectedActor` null (`/Game/CityBuilder/UI/Blueprints/HUD/WBP_HUD.WBP_SelectedBuildingMenu` _hudref))
  (`PrimitiveComponent.SetRenderCustomDepth` (`self.MeshRef`) false)
  (`/Game/CityBuilder/UI/Blueprints/HUD/WBP_HUD.CloseSelectedBuildingMenu` _hudref))