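; BP_Selectable_Resource is a selectable component that handles clicking on resources in the city builder.
; On selection it fills the HUD's selected resource menu with the name and description, shows it and passes it the owning actor.
; It highlights the selection by raising the mesh material's Emissive parameter.
; Deselection hides the menu, clears its actor reference and resets the glow, while BeginPlay defers to the parent.
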(event `self.ReceiveBeginPlay`
  (`parent.ReceiveBeginPlay`))

(event `self.Selected`
  (bind _wbp_selectedresourcemenu (`/Game/CityBuilder/UI/Blueprints/HUD/WBP_HUD.WBP_SelectedResourceMenu` (`self.HUDRef`)))
  (set `self.bIsClicked?` true)
  (`TextBlock.SetText` (`/Game/CityBuilder/UI/Blueprints/HUD/WBP_SelectedResourceMenu.ObjectName` _wbp_selectedresourcemenu) (`self.ResourceName`))
  (`RichTextBlock.SetText` (`/Game/CityBuilder/UI/Blueprints/HUD/WBP_SelectedResourceMenu.ObjectDescription` _wbp_selectedresourcemenu) (`self.ResourceDescription`))
  (`Widget.SetVisibility` _wbp_selectedresourcemenu "Visible")
  (set `/Game/CityBuilder/UI/Blueprints/HUD/WBP_SelectedResourceMenu.SelectedActor` (`self.OwningActor`) _wbp_selectedresourcemenu)
  (`MaterialInstanceDynamic.SetScalarParameterValue` (`self.MeshMaterial`) "Emissive" 0.5))

(event `self.Deselected`
  (bind _wbp_selectedresourcemenu (`/Game/CityBuilder/UI/Blueprints/HUD/WBP_HUD.WBP_SelectedResourceMenu` (`self.HUDRef`)))
  (set `self.bIsClicked?` false)
  (`Widget.SetVisibility` _wbp_selectedresourcemenu "Hidden")
  (set `/Game/CityBuilder/UI/Blueprints/HUD/WBP_SelectedResourceMenu.SelectedActor` null _wbp_selectedresourcemenu)
  (`MaterialInstanceDynamic.SetScalarParameterValue` (`self.MeshMaterial`) "Emissive" 0.0))