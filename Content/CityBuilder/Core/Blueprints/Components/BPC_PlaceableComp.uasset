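; Actor component for a city builder's placement preview that checks every tick whether the building can be placed.
; Four short downward corner traces flag edges, obstructions and water.
; That result combines with the player controller's affordability flag and an overlap check against other buildings to set validity.
; It swaps the owner mesh's material between valid and invalid and writes the failure reason to the owner's warning widget.
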(event `self.ReceiveBeginPlay`
  (bind _aspc_city_builder_player (cast `/Game/CityBuilder/Core/Blueprints/Player/PC_CityBuilderPlayer` (`GameplayStatics.GetPlayerController` 0)))
  (set `self.PlayerController` _aspc_city_builder_player)
  (bind _aswbp_placement_warning_widget (cast `/Game/CityBuilder/UI/Blueprints/InWorld/WBP_PlacementWarningWidget` (`WidgetComponent.GetWidget` (`Actor.GetComponentByClass` (`self.GetOwner`) "/Script/UMG.WidgetComponent"))))
  (set `self.WarningWidget` _aswbp_placement_warning_widget))

(event `self.ReceiveTick`
  (params (DeltaSeconds :type "Float (single-precision)"))
  (`self.LineTraces`)
  (`self.UpdateState`))

(fn `LineTraces`
  (bind _tracelocation (`self.TraceLocation`))
  (bind _warningwidget (`self.WarningWidget`))
  (bind _returnvalue (* _tracelocation -1.0))
  (for _index (range 4)
    (bind _returnvalue_2 (+ (`SceneComponent.K2_GetComponentLocation` (`Actor.GetComponentByClass` (`self.GetOwner`) "/Script/Engine.StaticMeshComponent")) (`KismetMathLibrary.MakeVector` (select `int` _index :`0` _returnvalue :`1` _tracelocation :`2` _tracelocation :`3` _returnvalue) (select `int` _index :`0` _tracelocation :`1` _tracelocation :`2` _returnvalue :`3` _returnvalue) 25.0)))
    (bind _outhit (`KismetSystemLibrary.LineTraceSingle` :`Start` _returnvalue_2 :`End` (- _returnvalue_2 (0.0 0.0 35.0)) :`TraceChannel` "TraceTypeQuery3" :`DrawDebugType` "ForOneFrame" :`DrawTime` 1.0))
    (bind (_bblockinghit _binitialoverlap _time _distance _location _impactpoint _normal _impactnormal _physmat _hitactor _hitcomponent) (`GameplayStatics.BreakHitResult` _outhit))
    (if _bblockinghit
      (if (> _distance 10.0)
        (if (`self.ComponentHasTag` _hitcomponent "Water")
          (set `/Game/CityBuilder/UI/Blueprints/InWorld/WBP_PlacementWarningWidget.WarningText` "Building cannot be placed in water!" _warningwidget)
          (set `self.bTracesValid?` false :!label _label)
          (return))
        (else
          (set `/Game/CityBuilder/UI/Blueprints/InWorld/WBP_PlacementWarningWidget.WarningText` "Building obstructed!" _warningwidget)
          (goto _label)))
      (else
        (set `/Game/CityBuilder/UI/Blueprints/InWorld/WBP_PlacementWarningWidget.WarningText` "Too close to edge!" _warningwidget)
        (goto _label))))
  (set `self.bTracesValid?` true)
  (set `/Game/CityBuilder/UI/Blueprints/InWorld/WBP_PlacementWarningWidget.WarningText` "" (`self.WarningWidget`))
  (return))

(fn `UpdateState`
  (bind _returnvalue (`self.GetOwner`))
  (bind _warningwidget (`self.WarningWidget`))
  (bind _returnvalue_2 (`Actor.GetComponentByClass` _returnvalue "/Script/Engine.StaticMeshComponent"))
  (bind _bcanafford_ (`/Game/CityBuilder/Core/Blueprints/Player/PC_CityBuilderPlayer.bCanAfford?` (`self.PlayerController`)))
  (bind _returnvalue_3 (== (`KismetArrayLibrary.Array_Length` (`Actor.GetOverlappingActors` _returnvalue "/Game/CityBuilder/Core/Blueprints/Actors/Buidings/BP_Building_Base.BP_Building_Base_C")) 0))
  (bind _output_get (set `self.bIsPlacementValid?` (and (`self.bTracesValid?`) _bcanafford_ _returnvalue_3)))
  (if (and _output_get _bcanafford_)
    (`PrimitiveComponent.SetMaterial` _returnvalue_2 0 (`self.PlaceableMaterial`))
    (else
      (`PrimitiveComponent.SetMaterial` _returnvalue_2 0 (`self.InvalidPlaceableMaterial`))
      (if _bcanafford_
        (if (not _returnvalue_3)
          (set `/Game/CityBuilder/UI/Blueprints/InWorld/WBP_PlacementWarningWidget.WarningText` "Building too close!" _warningwidget))
        (else
          (set `/Game/CityBuilder/UI/Blueprints/InWorld/WBP_PlacementWarningWidget.WarningText` "Can't afford!" _warningwidget))))))