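; Placement component for the farm in the city builder, overriding the state check that decides whether the farm can be placed.
; UpdateState requires valid traces and no other buildings overlapping the owner's second static mesh, which serves as a clearance volume.
; That result and the player controller's affordability flag switch the first mesh between placeable and invalid materials.
; On failure it sets the warning text, with affordability taking priority over spacing.
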(event `self.ReceiveTick`
  (params (DeltaSeconds :type "Float (single-precision)"))
  (`parent.ReceiveTick` DeltaSeconds))

(fn `UpdateState`
  (bind _warningwidget (`self.WarningWidget`))
  (bind _returnvalue (`Actor.K2_GetComponentsByClass` (`self.GetOwner`) "/Script/Engine.StaticMeshComponent"))
  (bind _bcanafford_ (`/Game/CityBuilder/Core/Blueprints/Player/PC_CityBuilderPlayer.bCanAfford?` (`self.PlayerController`)))
  (bind _output (`|GetArrayItem` _returnvalue))
  (bind _output_get (set `self.bIsPlacementValid?` (and (`self.bTracesValid?`) (== (`KismetArrayLibrary.Array_Length` (`PrimitiveComponent.GetOverlappingActors` (`|GetArrayItem` _returnvalue 1) "/Game/CityBuilder/Core/Blueprints/Actors/Buidings/BP_Building_Base.BP_Building_Base_C")) 0))))
  (if (and _output_get _bcanafford_)
    (`PrimitiveComponent.SetMaterial` _output 0 (`self.PlaceableMaterial`))
    (else
      (`PrimitiveComponent.SetMaterial` _output 0 (`self.InvalidPlaceableMaterial`))
      (if _bcanafford_
        (if (not _output_get)
          (set `/Game/CityBuilder/UI/Blueprints/InWorld/WBP_PlacementWarningWidget.WarningText` "Building too close!" _warningwidget))
        (else
          (set `/Game/CityBuilder/UI/Blueprints/InWorld/WBP_PlacementWarningWidget.WarningText` "Can't afford!" _warningwidget))))))