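; Placeable component for docks in the city builder that updates buff and placement validity in UpdateState.
; Market overlaps on the owner's first mesh set the buff multiplier, which drops as markets increase and feeds buff widgets.
; Validity requires parent trace checks, no building overlap on the second mesh, and a downward side-offset trace hitting a Water-tagged component.
; Validity and affordability drive the highlight color through a material parameter collection, plus warning text.
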(fn `UpdateState`
  (bind _returnvalue (`self.GetOwner`))
  (bind _warningwidget (`self.WarningWidget`))
  (bind _bcanafford_ (`/Game/CityBuilder/Core/Blueprints/Player/PC_CityBuilderPlayer.bCanAfford?` (`self.PlayerController`)))
  (bind _overlappingactors (`PrimitiveComponent.GetOverlappingActors` (`|GetArrayItem` (`Actor.K2_GetComponentsByClass` (`self.GetOwner`) "/Script/Engine.StaticMeshComponent")) "/Game/CityBuilder/Core/Blueprints/Actors/Buidings/BP_Building_Market.BP_Building_Market_C"))
  (bind _returnvalue_2 (`KismetArrayLibrary.Array_Length` _overlappingactors))
  (bind _returnvalue_3 (+ (+ (`Actor.K2_GetActorLocation` _returnvalue) (* (`Actor.GetActorRightVector` _returnvalue) 750.0)) (0.0 0.0 50.0)))
  (bind _returnvalue_4 (== (`KismetArrayLibrary.Array_Length` (`PrimitiveComponent.GetOverlappingActors` (`|GetArrayItem` (`Actor.K2_GetComponentsByClass` _returnvalue "/Script/Engine.StaticMeshComponent") 1) "/Game/CityBuilder/Core/Blueprints/Actors/Buidings/BP_Building_Base.BP_Building_Base_C")) 0))
  (if (== _returnvalue_2 0)
    (set `self.BuffMultiplier` 2)
    (else
      (for _array_element _overlappingactors
        (bind _asbp_in_world_base (cast `/Game/CityBuilder/Core/Blueprints/BP_InWorld_Base` _array_element))
        (set `/Game/CityBuilder/Core/Blueprints/BP_InWorld_Base.BuffMultIndicator` (`self.BuffMultiplier`) _asbp_in_world_base)
        (`/Game/CityBuilder/Core/Blueprints/BP_InWorld_Base.CreateBuffWidget` _asbp_in_world_base false)
        (set `self.BuffMultiplier` 1))
      (if (>= _returnvalue_2 3)
        (set `self.BuffMultiplier` 0))))
  (bind _asbp_dummy_building (cast `/Game/CityBuilder/Core/Blueprints/Actors/Buidings/BP_DummyBuilding` (`self.GetOwner`))
    (:`then`
      (set `/Game/CityBuilder/Core/Blueprints/Actors/Buidings/BP_DummyBuilding.BuffMultiplierPasstrough` (`self.BuffMultiplier`) _asbp_dummy_building)
      (`/Game/CityBuilder/Core/Blueprints/Actors/Buidings/BP_DummyBuilding.CreateBuffWidget` _asbp_dummy_building))
    (:`CastFailed`
      _))
  (bind _outhit (`KismetSystemLibrary.LineTraceSingle` :`Start` _returnvalue_3 :`End` (- _returnvalue_3 (0.0 0.0 200.0)) :`TraceChannel` "TraceTypeQuery3" :`DrawDebugType` "ForDuration" :`DrawTime` 1.0))
  (bind (_bblockinghit _binitialoverlap _time _distance _location _impactpoint _normal _impactnormal _physmat _hitactor _hitcomponent) (`GameplayStatics.BreakHitResult` _outhit))
  (if _bblockinghit
    (bind _returnvalue_5 (`self.ComponentHasTag` _hitcomponent "Water"))
    (bind _output_get (set `self.bIsPlacementValid?` (and (`self.bTracesValid?`) (and _returnvalue_4 _returnvalue_5))))
    (if (and _output_get _bcanafford_)
      (`KismetMaterialLibrary.SetVectorParameterValue` "/Game/CityBuilder/Core/Data/ParameterCollections/MPC_UIColors.MPC_UIColors" "HighlightColor" (make `LinearColor` 1.5 1.5 1.5 1.0))
      (else
        (`KismetMaterialLibrary.SetVectorParameterValue` "/Game/CityBuilder/Core/Data/ParameterCollections/MPC_UIColors.MPC_UIColors" "HighlightColor" (`self.InvalidPlacementColor`))
        (if _bcanafford_
          (if _returnvalue_4
            (if (and _bblockinghit (not _returnvalue_5))
              (set `/Game/CityBuilder/UI/Blueprints/InWorld/WBP_PlacementWarningWidget.WarningText` "Needs to be near water!" _warningwidget :!label _label))
            (else
              (set `/Game/CityBuilder/UI/Blueprints/InWorld/WBP_PlacementWarningWidget.WarningText` "Building too close!" _warningwidget)))
          (else
            (set `/Game/CityBuilder/UI/Blueprints/InWorld/WBP_PlacementWarningWidget.WarningText` "Can't afford!" _warningwidget)))))
    (else
      (goto _label))))