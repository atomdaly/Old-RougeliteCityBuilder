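; Placement component for the city builder's mine, which validates where the building preview can be placed.
; Its UpdateState requires valid traces, no overlapping buildings and at least one overlapping stone resource.
; It swaps the owner mesh's material according to validity and the player's ability to afford it.
; On failure it sets warning widget text for cost, building proximity or missing stone, with affordability taking priority.
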(event `self.ReceiveTick`
  (params (DeltaSeconds :type "Float (single-precision)"))
  (`parent.ReceiveTick` DeltaSeconds))

(fn `UpdateState`
  (bind _returnvalue (`self.GetOwner`))
  (bind _warningwidget (`self.WarningWidget`))
  (bind _returnvalue_2 (`Actor.GetComponentByClass` _returnvalue "/Script/Engine.StaticMeshComponent"))
  (bind _bcanafford_ (`/Game/CityBuilder/Core/Blueprints/Player/PC_CityBuilderPlayer.bCanAfford?` (`self.PlayerController`)))
  (bind _returnvalue_3 (== (`KismetArrayLibrary.Array_Length` (`Actor.GetOverlappingActors` _returnvalue "/Game/CityBuilder/Core/Blueprints/Actors/Buidings/BP_Building_Base.BP_Building_Base_C")) 0))
  (bind _returnvalue_4 (>= (`KismetArrayLibrary.Array_Length` (`Actor.GetOverlappingActors` _returnvalue "/Game/CityBuilder/Core/Blueprints/Actors/Resources/BP_Resource_Stone.BP_Resource_Stone_C")) 1))
  (bind _output_get (set `self.bIsPlacementValid?` (and (`self.bTracesValid?`) (and _returnvalue_3 _returnvalue_4))))
  (if (and _output_get _bcanafford_)
    (`PrimitiveComponent.SetMaterial` _returnvalue_2 0 (`self.PlaceableMaterial`))
    (else
      (`PrimitiveComponent.SetMaterial` _returnvalue_2 0 (`self.InvalidPlaceableMaterial`))
      (if _bcanafford_
        (if _returnvalue_3
          (if (not _returnvalue_4)
            (set `/Game/CityBuilder/UI/Blueprints/InWorld/WBP_PlacementWarningWidget.WarningText` "Needs to be near stone!" _warningwidget))
          (else
            (set `/Game/CityBuilder/UI/Blueprints/InWorld/WBP_PlacementWarningWidget.WarningText` "Building too close!" _warningwidget)))
        (else
          (set `/Game/CityBuilder/UI/Blueprints/InWorld/WBP_PlacementWarningWidget.WarningText` "Can't afford!" _warningwidget))))))