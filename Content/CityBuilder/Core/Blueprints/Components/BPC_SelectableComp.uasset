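; BPC_SelectableComp is a base component that makes in-world city builder actors hoverable and clickable for selection outside placement mode.
; Hovering toggles the mesh's custom depth unless the actor is selected.
; Clicking toggles selection, first deselecting whichever actor the HUD's building or resource menu holds.
; Selected and Deselected are empty hooks, and BeginPlay caches the controller, mesh, dynamic material and HUD, the last after a short delay.
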(event `self.ReceiveBeginPlay`
  (bind _returnvalue (`self.GetOwner`))
  (bind _returnvalue_2 (`Actor.GetComponentByClass` _returnvalue "/Script/Engine.StaticMeshComponent"))
  (bind _aspc_city_builder_player (cast `/Game/CityBuilder/Core/Blueprints/Player/PC_CityBuilderPlayer` (`GameplayStatics.GetPlayerController` 0)))
  (set `self.PlayerController` _aspc_city_builder_player)
  (add `Actor.OnClicked` _returnvalue (delegate `OnMouseClicked`))
  (`/Engine/EditorBlueprintResources/StandardMacros.IsValid` _returnvalue_2
    (:`Is Valid`
      (set `self.MeshRef` _returnvalue_2)
      (bind _asbp_in_world_base (cast `/Game/CityBuilder/Core/Blueprints/BP_InWorld_Base` (`self.GetOwner`)))
      (set `self.OwningActor` _asbp_in_world_base)
      (add `Actor.OnBeginCursorOver` _returnvalue (delegate `OnMouseHover`))
      (add `Actor.OnEndCursorOver` _returnvalue (delegate `OnMouseHoverEnd`))
      (bind _returnvalue_3 (`PrimitiveComponent.CreateDynamicMaterialInstance` (`self.MeshRef`) 0 "/Game/CityBuilder/Art/Materials/Environment/M_BaseMaterial.M_BaseMaterial" "None"))
      (set `self.MeshMaterial` _returnvalue_3)
      (`KismetSystemLibrary.Delay` 0.2)
      (bind _foundwidgets (`WidgetBlueprintLibrary.GetAllWidgetsOfClass` "/Game/CityBuilder/UI/Blueprints/HUD/WBP_HUD.WBP_HUD_C"))
      (set `self.HUDRef` (`|GetArrayItem` _foundwidgets)))))

(event `OnMouseHover`
  (params (TouchedActor :type "Actor Object Reference"))
  (if (not (or (`/Game/CityBuilder/Core/Blueprints/Player/PC_CityBuilderPlayer.bPlacementModeEnabled?` (`self.PlayerController`)) (`self.bIsClicked?`)))
    (`PrimitiveComponent.SetRenderCustomDepth` (`self.MeshRef`) true)))

(event `OnMouseHoverEnd`
  (params (TouchedActor :type "Actor Object Reference"))
  (if (not (or (`/Game/CityBuilder/Core/Blueprints/Player/PC_CityBuilderPlayer.bPlacementModeEnabled?` (`self.PlayerController`)) (`self.bIsClicked?`)))
    (`PrimitiveComponent.SetRenderCustomDepth` (`self.MeshRef`) false)))

(event `OnMouseClicked`
  (params (TouchedActor :type "Actor Object Reference") (ButtonPressed :type "Key Structure" :default "None"))
  (bind _hudref (`self.HUDRef`))
  (bind _selectedactor (`/Game/CityBuilder/UI/Blueprints/HUD/WBP_SelectedBuildingMenu.SelectedActor` (`/Game/CityBuilder/UI/Blueprints/HUD/WBP_HUD.WBP_SelectedBuildingMenu` _hudref)))
  (bind _selectedactor_2 (`/Game/CityBuilder/UI/Blueprints/HUD/WBP_SelectedResourceMenu.SelectedActor` (`/Game/CityBuilder/UI/Blueprints/HUD/WBP_HUD.WBP_SelectedResourceMenu` _hudref)))
  (if (not (`/Game/CityBuilder/Core/Blueprints/Player/PC_CityBuilderPlayer.bPlacementModeEnabled?` (`self.PlayerController`)))
    (bind _output_get (set `self.bIsClicked?` (not (`self.bIsClicked?`))))
    (`/Engine/EditorBlueprintResources/StandardMacros.IsValid` (`self.MeshRef`)
      (:`Is Valid`
        (if _output_get
          (`/Engine/EditorBlueprintResources/StandardMacros.IsValid` _selectedactor
            (:`Is Valid`
              (`self.Deselected` (`Actor.GetComponentByClass` _selectedactor "BPC_SelectableComp_C")))
            (:`Is Not Valid`
              (`/Engine/EditorBlueprintResources/StandardMacros.IsValid` _selectedactor_2
                (:`Is Valid`
                  (`self.Deselected` (`Actor.GetComponentByClass` _selectedactor_2 "BPC_SelectableComp_C")))
                (:`Is Not Valid`
                  _))))
          (`KismetSystemLibrary.Delay` 0.1)
          (`self.Selected`)
          (else
            (`self.Deselected`)))))))

(event `Selected`)

(event `Deselected`)