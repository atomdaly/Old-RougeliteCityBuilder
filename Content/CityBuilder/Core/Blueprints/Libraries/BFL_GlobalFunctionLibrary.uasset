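; BFL_GlobalFunctionLibrary is the city builder's global function library, holding the GameEndCheck function that detects a lost game.
; It reads population balance and happiness percent from the first player's PC_CityBuilderPlayer controller.
; If either is zero or below, it pauses the game and shows WBP_GameOverScreen with the reason, with population loss taking priority over low happiness.
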(fn `GameEndCheck`
  (bind _aspc_city_builder_player (cast `/Game/CityBuilder/Core/Blueprints/Player/PC_CityBuilderPlayer` (`GameplayStatics.GetPlayerController` null)))
  (bind _returnvalue (<= (`/Game/CityBuilder/Core/Blueprints/Player/PC_CityBuilderPlayer.PopulationBalance` _aspc_city_builder_player) 0))
  (if (or _returnvalue (<= (`/Game/CityBuilder/Core/Blueprints/Player/PC_CityBuilderPlayer.HappinessPercent` _aspc_city_builder_player) 0))
    (`GameplayStatics.SetGamePaused` null true)
    (bind _returnvalue_2 (`|CreateWidget` "/Game/CityBuilder/UI/Blueprints/HUD/WBP_GameOverScreen.WBP_GameOverScreen_C"))
    (`TextBlock.SetText` (`/Game/CityBuilder/UI/Blueprints/HUD/WBP_GameOverScreen.ReasonText` _returnvalue_2) (`KismetTextLibrary.Conv_StringToText` (`KismetStringLibrary.Concat_StrStr` "(" (`KismetMathLibrary.SelectString` "Lost all your people" "Happiness too low" _returnvalue) ")")))
    (`UserWidget.AddToViewport` _returnvalue_2 0)))