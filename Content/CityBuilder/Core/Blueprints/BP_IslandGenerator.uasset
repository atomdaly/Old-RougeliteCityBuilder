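; Procedural island generator for the city-builder, populating randomized terrain with resources and foliage.
; Construction and BeginPlay rebuild the island from random terrain slab meshes plus a sand plane.
; BeginPlay then uses random line traces to spawn a capped number of resource actors off water, validated by four corner traces.
; Further traces scatter grass and tree instanced meshes on near-flat Terrain-tagged surfaces.
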(event `self.ReceiveBeginPlay`
  (`self.RandomlyGenerateIsland`)
  (`self.SpawnResources`)
  (`self.SpawnFoliage`))

(fn `RandomlyGenerateIsland`
  (bind _returnvalue (`KismetMathLibrary.RandomFloatInRange` 0.0 360.0))
  (bind _returnvalue_2 (`KismetMathLibrary.RandomFloatInRange` 1.0 1.25))
  (bind _returnvalue_3 (`KismetMathLibrary.RandomFloatInRange` 1.0 1.25))
  (bind _islandpositions (`self.IslandPositions`))
  (bind _islandsmaxdistance (`self.IslandsMaxDistance`))
  (bind _islandsmaxdistance_2 (`self.IslandsMaxDistance`))
  (bind _returnvalue_4 (mod _returnvalue 45.0))
  (bind _returnvalue_5 (- _returnvalue _returnvalue_4))
  (bind (_arrayindex _arrayelement) (`/Engine/EditorBlueprintResources/StandardMacros.ReverseForEachLoop` (`self.K2_GetComponentsByClass` "/Script/Engine.StaticMeshComponent"))
    (:`LoopBody`
      (`ActorComponent.K2_DestroyComponent` _arrayelement))
    (:`Completed`
      (for _ (range (+ (`KismetMathLibrary.RandomIntegerInRange` 1 3) 1))
        (for _array_element _islandpositions :!label _label
          (bind _output_get (set `self.IslandPosition` (`KismetMathLibrary.RandomFloatInRange` (* _islandsmaxdistance_2 -1.0) _islandsmaxdistance_2)))
          (if (`KismetMathLibrary.NearlyEqual_FloatFloat` _output_get _array_element 1000.0)
            (goto _label)
            (else
              (break))))
        (bind _returnvalue_6 (`KismetArrayLibrary.Array_Add` _islandpositions (`self.IslandPosition`)))
        (`KismetSystemLibrary.PrintString` (`KismetStringLibrary.Conv_DoubleToString` (`|GetArrayItem` (`self.IslandPositions`) _returnvalue_6)) true false (struct :`R` 0.114192 :`G` 1.0 :`A` 1.0))
        (bind _returnvalue_7 (`AddComponent|NODE_AddStaticMeshComponent-0` :`RelativeTransform` (`KismetMathLibrary.MakeTransform` (`KismetMathLibrary.MakeVector` (`self.IslandPosition`) (`KismetMathLibrary.RandomFloatInRange` (* _islandsmaxdistance -1.0) _islandsmaxdistance)) (`KismetMathLibrary.MakeRotator` 0.0 0.0 (`KismetMathLibrary.RandomFloatInRange` 0.0 360.0)) (`KismetMathLibrary.MakeVector` _returnvalue_3 _returnvalue_3 1.0))))
        (`StaticMeshComponent.SetStaticMesh` _returnvalue_7 (select `int` (`KismetMathLibrary.RandomIntegerInRange` 0 3) :`0` "/Game/CityBuilder/Art/3D/Environment/Terrain/SM_TerrainSlab_01.SM_TerrainSlab_01" :`1` "/Game/CityBuilder/Art/3D/Environment/Terrain/SM_TerrainSlab_02.SM_TerrainSlab_02" :`2` "/Game/CityBuilder/Art/3D/Environment/Terrain/SM_TerrainSlab_03.SM_TerrainSlab_03" :`3` "/Game/CityBuilder/Art/3D/Environment/Terrain/SM_TerrainSlab_04.SM_TerrainSlab_04" :!type "StaticMesh Object Reference")))
      (bind _returnvalue_8 (`AddComponent|NODE_AddStaticMeshComponent-3` :`RelativeTransform` (`KismetMathLibrary.MakeTransform` (0.0 0.0 -250.0) (`KismetMathLibrary.MakeRotator` 0.0 0.0 (select `bool` (< _returnvalue_4 22.5) :`false` _returnvalue_5 :`true` (+ _returnvalue_5 45.0))) (`KismetMathLibrary.MakeVector` _returnvalue_2 _returnvalue_2 1.0))))
      (`StaticMeshComponent.SetStaticMesh` _returnvalue_8 (select `int` (`KismetMathLibrary.RandomIntegerInRange` 0 3) :`0` "/Game/CityBuilder/Art/3D/Environment/Terrain/SM_SandPlane_01.SM_SandPlane_01" :`1` "/Game/CityBuilder/Art/3D/Environment/Terrain/SM_SandPlane_02.SM_SandPlane_02" :`2` "/Game/CityBuilder/Art/3D/Environment/Terrain/SM_SandPlane_03.SM_SandPlane_03" :`3` "/Game/CityBuilder/Art/3D/Environment/Terrain/SM_SandPlane_04.SM_SandPlane_04" :!type "StaticMesh Object Reference")))))

(fn `SpawnCheckTraces`
  (params (MainHitLocation :type "Vector Structure"))
  (returns (`bValidLocation?` :type Boolean))
  (bind _tracelocation (`self.TraceLocation`))
  (bind _returnvalue (* _tracelocation -1.0))
  (for _index (range 4)
    (bind _returnvalue_2 (+ MainHitLocation (`KismetMathLibrary.MakeVector` (select `int` _index :`0` _returnvalue :`1` _tracelocation :`2` _tracelocation :`3` _returnvalue) (select `int` _index :`0` _tracelocation :`1` _tracelocation :`2` _returnvalue :`3` _returnvalue) 50.0)))
    (bind _outhit (`KismetSystemLibrary.LineTraceSingle` :`Start` _returnvalue_2 :`End` (- _returnvalue_2 (0.0 0.0 75.0)) :`TraceChannel` "TraceTypeQuery1" :`DrawDebugType` "ForDuration" :`bIgnoreSelf` false :`TraceColor` (struct :`R` 0.848742 :`B` 1.0 :`A` 1.0) :`TraceHitColor` (struct :`R` 1.0 :`G` 0.861242 :`A` 1.0) :`DrawTime` 25.0))
    (bind (_bblockinghit _binitialoverlap _time _distance) (`GameplayStatics.BreakHitResult` _outhit))
    (if (and _bblockinghit (> _distance 10.0))
      (bind _returnvalue_3 (== _index 3))
      (if _returnvalue_3
        (return _returnvalue_3))
      (else
        (return false)))))

(fn `SpawnFoliage`
  (bind _returnvalue (`KismetMathLibrary.RandomFloatInRange` -6000.0 6000.0))
  (bind _returnvalue_2 (`KismetMathLibrary.RandomFloatInRange` -6000.0 6000.0))
  (bind _returnvalue_3 (`KismetMathLibrary.RandomFloatInRange` -6000.0 6000.0))
  (bind _returnvalue_4 (`KismetMathLibrary.RandomFloatInRange` -6000.0 6000.0))
  (bind _returnvalue_5 (`AddComponent|NODE_AddInstancedStaticMeshComponent-0`))
  (set `self.TreeISMComponent` _returnvalue_5)
  (bind _returnvalue_6 (`AddComponent|NODE_AddInstancedStaticMeshComponent-1`))
  (set `self.GrassISMComponent` _returnvalue_6)
  (for _ (range 1001)
    (bind _outhit (`KismetSystemLibrary.LineTraceSingle` :`Start` (`KismetMathLibrary.MakeVector` _returnvalue_4 _returnvalue_3 5000.0) :`End` (`KismetMathLibrary.MakeVector` _returnvalue_4 _returnvalue_3 250.0) :`TraceChannel` "TraceTypeQuery1" :`bIgnoreSelf` false :`TraceColor` (struct :`R` 0.369605 :`G` 1.0 :`A` 1.0) :`TraceHitColor` (struct :`G` 1.0 :`B` 0.510704 :`A` 1.0)))
    (bind (_bblockinghit _binitialoverlap _time _distance _location _impactpoint _normal _impactnormal _physmat _hitactor) (`GameplayStatics.BreakHitResult` _outhit))
    (if (and _bblockinghit (> (.z _impactnormal) 0.8))
      (if (`self.ActorHasTag` _hitactor "Terrain")
        (`InstancedStaticMeshComponent.AddInstance` (`self.GrassISMComponent`) (`KismetMathLibrary.MakeTransform` _location (`KismetMathLibrary.MakeRotator` 0.0 0.0 (`KismetMathLibrary.RandomFloatInRange` 0.0 360.0))) false))))
  (for _ (range 51)
    (bind _outhit_2 (`KismetSystemLibrary.LineTraceSingle` :`Start` (`KismetMathLibrary.MakeVector` _returnvalue _returnvalue_2 5000.0) :`End` (`KismetMathLibrary.MakeVector` _returnvalue _returnvalue_2 250.0) :`TraceChannel` "TraceTypeQuery1" :`bIgnoreSelf` false :`TraceColor` (struct :`R` 0.369605 :`G` 1.0 :`A` 1.0) :`TraceHitColor` (struct :`G` 1.0 :`B` 0.510704 :`A` 1.0)))
    (bind (_bblockinghit_2 _binitialoverlap_2 _time_2 _distance_2 _location_2 _impactpoint_2 _normal_2 _impactnormal_2 _physmat_2 _hitactor_2) (`GameplayStatics.BreakHitResult` _outhit_2))
    (if (and _bblockinghit_2 (> (.z _impactnormal_2) 0.8))
      (if (`self.ActorHasTag` _hitactor_2 "Terrain")
        (`InstancedStaticMeshComponent.AddInstance` (`self.TreeISMComponent`) (`KismetMathLibrary.MakeTransform` _location_2 (`KismetMathLibrary.MakeRotator` 0.0 0.0 (`KismetMathLibrary.RandomFloatInRange` 0.0 360.0))) false)))))

(fn `SpawnResources`
  (locals (NumberOfResources :type Integer))
  (bind _returnvalue (`KismetMathLibrary.RandomFloatInRange` -6000.0 6000.0))
  (bind _returnvalue_2 (`KismetMathLibrary.RandomFloatInRange` -6000.0 6000.0))
  (for _ (range 101)
    (if (<= (`local.NumberOfResources`) 4)
      (bind _outhit (`KismetSystemLibrary.LineTraceSingle` :`Start` (`KismetMathLibrary.MakeVector` _returnvalue_2 _returnvalue 5000.0) :`End` (`KismetMathLibrary.MakeVector` _returnvalue_2 _returnvalue) :`TraceChannel` "TraceTypeQuery1" :`bIgnoreSelf` false :`TraceColor` (struct :`R` 0.369605 :`G` 1.0 :`A` 1.0) :`TraceHitColor` (struct :`G` 1.0 :`B` 0.510704 :`A` 1.0)))
      (bind (_bblockinghit _binitialoverlap _time _distance _location _impactpoint _normal _impactnormal _physmat _hitactor _hitcomponent) (`GameplayStatics.BreakHitResult` _outhit))
      (if _bblockinghit
        (if (not (`ActorComponent.ComponentHasTag` _hitcomponent "Water"))
          (bind _bvalidlocation_ (`self.SpawnCheckTraces` _location))
          (if _bvalidlocation_
            (bind _returnvalue_3 (`|SpawnActorFromClass` (`KismetArrayLibrary.Array_Random` (`self.Resources`)) (`KismetMathLibrary.MakeTransform` _location (`KismetMathLibrary.MakeRotator` 0.0 0.0 (`KismetMathLibrary.RandomFloatInRange` 0.0 340.0))) "Undefined" "OverrideRootScale" null null))
            (if (== (`KismetArrayLibrary.Array_Length` (`self.GetOverlappingActors` _returnvalue_3 "/Game/CityBuilder/Core/Blueprints/BP_InWorld_Base.BP_InWorld_Base_C")) 0)
              (`/Engine/EditorBlueprintResources/StandardMacros.IncrementInt` (`local.NumberOfResources`))))))
      (else
        (break)))))

(fn `UserConstructionScript`
  (`self.RandomlyGenerateIsland`))