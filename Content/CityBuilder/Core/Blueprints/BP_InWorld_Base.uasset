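; Base in-world actor for the city builder that shows a neighbour buff indicator while a dummy building overlaps it.
; BeginPlay caches the player controller, game state and island generator.
; Overlap begin adds a widget component with rich-text "+1" chosen by currency type, and overlap end destroys it.
; WidgetButtonClicked is an empty stub, BaseMesh overlap only debug-prints the hit item, and instance-removal nodes sit disconnected.
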(event `self.ReceiveBeginPlay`
  (bind _aspc_city_builder_player (cast `/Game/CityBuilder/Core/Blueprints/Player/PC_CityBuilderPlayer` (`GameplayStatics.GetPlayerController` 0)))
  (set `self.PlayerController` _aspc_city_builder_player)
  (bind _asgs_city_builder_game_state (cast `/Game/CityBuilder/Core/Blueprints/GS_CityBuilderGameState` (`GameplayStatics.GetGameState`)))
  (set `self.GameState` _asgs_city_builder_game_state)
  (bind _returnvalue (`GameplayStatics.GetActorOfClass` "/Game/CityBuilder/Core/Blueprints/BP_IslandGenerator.BP_IslandGenerator_C"))
  (set `self.IslandGenerator` _returnvalue))

(event `WidgetButtonClicked`)

(event `DestroyWidgetComp`
  (bind _widgetcomp (`self.WidgetComp`))
  (`/Engine/EditorBlueprintResources/StandardMacros.IsValid` _widgetcomp
    (:`Is Valid`
      (`ActorComponent.K2_DestroyComponent` _widgetcomp))))

(event `self.ReceiveActorEndOverlap`
  (params (OtherActor :type "Actor Object Reference"))
  (if (== (`GameplayStatics.GetObjectClass` OtherActor) "/Game/CityBuilder/Core/Blueprints/Actors/Buidings/BP_DummyBuilding.BP_DummyBuilding_C")
    (`self.DestroyWidgetComp`)))

(event `self.ReceiveActorBeginOverlap`
  (params (OtherActor :type "Actor Object Reference"))
  (if (== (`GameplayStatics.GetObjectClass` OtherActor) "/Game/CityBuilder/Core/Blueprints/Actors/Buidings/BP_DummyBuilding.BP_DummyBuilding_C")
    (`self.CreateBuffWidget`)))

(event `self.BaseMesh.OnComponentBeginOverlap`
  (params (OverlappedComponent :type "PrimitiveComponent Object Reference") (OtherActor :type "Actor Object Reference") (OtherComp :type "PrimitiveComponent Object Reference") (OtherBodyIndex :type Integer) (bFromSweep :type Boolean) (SweepResult :type "HitResult Structure (by ref)"))
  (`KismetSystemLibrary.PrintString` (`KismetStringLibrary.Conv_IntToString` (`.HitItem` (`GameplayStatics.BreakHitResult` SweepResult)))))

(fn `CreateBuffWidget`
  (returns (WidgetComp :type "WidgetComponent Object Reference"))
  (bind _returnvalue (`AddComponent|NODE_AddWidgetComponent-2`))
  (bind _output_get (set `self.WidgetComp` _returnvalue))
  (bind _aswbp_neighbour_buff_indicator (cast `/Game/CityBuilder/UI/Blueprints/InWorld/WBP_NeighbourBuffIndicator` (`WidgetComponent.GetWidget` _output_get)))
  (set `/Game/CityBuilder/UI/Blueprints/InWorld/WBP_NeighbourBuffIndicator.InText` (`KismetTextLibrary.Conv_StringToText` (select `/Game/CityBuilder/Core/Data/Enums/E_CurrencyTypes` (`self.CurrencyType`) :`NewEnumerator0` (`KismetStringLibrary.Concat_StrStr` "<TexPop>" "+1" "</> ") :`NewEnumerator1` (`KismetStringLibrary.Concat_StrStr` "<TexRes>" "+1" "</> ") :`NewEnumerator2` (`KismetStringLibrary.Concat_StrStr` "<TexProd>" "+1" "</> "))) _aswbp_neighbour_buff_indicator)
  (return _output_get))

(fn `UserConstructionScript`)