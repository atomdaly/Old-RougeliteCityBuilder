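; BP_MainMenuPawn is a main menu pawn holding unfinished, inactive logic for stepping between SettingsUI categories.
; Two disconnected chains find the top-level SettingsUI widget and bounds-check its CategorySwitcher index for next and previous steps.
; No event triggers either chain, the computed indices are unused, and the construction script is empty, so the graphs do nothing at runtime.
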(fn `UserConstructionScript`)